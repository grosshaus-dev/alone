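; BP_Ocean_Trigger is a water trigger actor that tells the player character when it enters or leaves the ocean.
; It caches player 0 as an AlonePlayerCharacter on BeginPlay.
; When that player begins overlapping WaterVolume, it sends UpdateWaterStateMessage with InWater true and the WaterSurface value.
; End overlap sends InWater false without checking which actor left, so any exiting overlap clears the player's water state.
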(event OnComponentBeginOverlap(WaterVolume)
  (params (OverlappedComponent :type Primitive%20Component%20Object%20Reference) (OtherActor :type Actor%20Object%20Reference) (OtherComp :type Primitive%20Component%20Object%20Reference) (OtherBodyIndex :type Integer) (bFromSweep :type Boolean) (SweepResult :type Hit%20Result%20Structure%20%28by%20ref%29))
  (if (== OtherActor (Variables|Default|GetPlayerCharacterReference))
    (Class|BPIPlayerCharacter|UpdateWaterState(Message) (Variables|Default|GetPlayerCharacterReference) (Variables|Default|GetWaterSurface) true)))

(event OnComponentEndOverlap(WaterVolume)
  (params (OverlappedComponent :type Primitive%20Component%20Object%20Reference) (OtherActor :type Actor%20Object%20Reference) (OtherComp :type Primitive%20Component%20Object%20Reference) (OtherBodyIndex :type Integer))
  (Class|BPIPlayerCharacter|UpdateWaterState(Message) (Variables|Default|GetPlayerCharacterReference) 0 false))

(event EventBeginPlay
  (bind _asalone_player_character (Utilities|Casting|CastToAlonePlayerCharacter (Game|GetPlayerCharacter 0)))
  (Variables|Default|SetPlayerCharacterReference _asalone_player_character))

(fn ConstructionScript)