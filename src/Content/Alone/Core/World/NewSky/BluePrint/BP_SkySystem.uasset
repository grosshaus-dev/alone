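; Sky system actor that drives sun, moon, sky material and exposure from game time.
; Once the player is ready, it reads monthly sunrise/sunset from climate data, and a timeline interpolates minutes to rotate both bodies via altitude/azimuth curves, with remapped twilight pitch.
; Sun height sets post-process brightness limits, and moon illumination picks the phase texture on a dynamic sky material.
; Tick also feeds sun direction to the player's shade check.
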(event EventBeginPlay
  (bind _returnvalue (Utilities|GetTimeOfDay))
  (bind _asalone_player_character (Utilities|Casting|CastToAlonePlayerCharacter (Game|GetPlayerCharacter 0)))
  (bind _output_get (Variables|Default|SetPlayerRef _asalone_player_character))
  ;[0.15 0.15 0.15 0.5] Wair for player character to be ready
  (if (Variables|/Game/Alone/Core/PlayerCharacter/AlonePlayerCharacter.AlonePlayerCharacter_C|GetReady _output_get) :!label _label
    (Variables|Default|SetGameTimeReference (Variables|/Game/Alone/Core/PlayerCharacter/AlonePlayerCharacter.AlonePlayerCharacter_C|GetGameTimeReference (Variables|Default|GetPlayerRef)))
    (Variables|Default|SetWeather%20Reference (Variables|/Game/Alone/Core/PlayerCharacter/AlonePlayerCharacter.AlonePlayerCharacter_C|GetWeatherReference (Variables|Default|GetPlayerRef)))
    (CallFunction|HandleCoordinates)
    (Variables|Default|SetSkyReady true)
    (Variables|Default|SetMinutesOfDay _returnvalue)
    (Variables|Default|SetTimeNext (+ _returnvalue 1.0))
    (else
      (Utilities|FlowControl|Delay 0.2)
      (goto _label))))

(event EventTick
  (params (DeltaSeconds :type Float%20%28single-precision%29))
  (bind _sun_height (Variables|Default|GetSun%20height))
  (bind _postprocessvolume (Variables|Default|GetPostProcessVolume))
  (bind _settings (Variables|/Script/Engine.PostProcessVolume|GetSettings _postprocessvolume))
  (bind (_autoexposureminbrightness _autoexposuremaxbrightness) (Utilities|Struct|BreakPostProcessSettings _settings))
  (if (Variables|Default|GetSkyReady)
    (Development|PrintString (Utilities|String|ToString(Float) (Variables|Default|GetSun%20height)) true true "(R=1.000000,G=0.810665,B=0.000000,A=1.000000)" 2.0 "5")
    (Utilities|FlowControl|Sequence
      (:then_0
        ;[0.15 0.15 0.15 0.5] Check if in shade
        (bind _asalone_player_character (Utilities|Casting|CastToAlonePlayerCharacter (Game|GetPlayerCharacter 0)))
        (Default|InShade _asalone_player_character (Math|Vector|GetForwardVector (Transformation|GetWorldRotation (Variables|/Script/Engine.Actor|GetRootComponent (Variables|Default|GetDirectional%20light%20actor))))))
      (:then_2
        ;[0.15 0.15 0.15 0.5] Handle Sun/Moon Rotation
        (Utilities|FlowControl|Gate false :!label _label
          (:Exit
            (Utilities|FlowControl|Sequence
              (:then_0
                (goto _label Close))
              (:then_1
                (Variables|Default|SetTimeNow (Utilities|GetTimeOfDay))
                (bind _2secconds (Timeline|TimelineNormal PlayFromStart)
                  (:Update
                    (Variables|Default|SetMinutesOfDay (Math|Float|Lerp (Variables|Default|GetTimeNow) (Variables|Default|GetTimeNext) _2secconds))
                    (CallFunction|HandleSunMoonRotation)
                    (CallFunction|RefreshMaterial))
                  (:Finished
                    (Variables|Default|SetTimeNext (+ (Utilities|GetTimeOfDay) 1.0))
                    (goto _label Open))))))))
      (:then_3
        (if (< (Variables|Default|GetSun%20height) 0.0)
          (Utilities|Struct|SetmembersinPostProcessSettings (Variables|/Script/Engine.PostProcessVolume|GetSettings (Variables|Default|GetPostProcessVolume)) (Math|Float|MapRangeClamped _sun_height 0.0 -1.0 1e+01 -2.0) (Math|Float|MapRangeClamped _sun_height 0.0 -1.0 14.0 1.0))
          (else
            (CallFunction|HandleDayNightCycle))))
      (:then_4
        (CallFunction|HandleMoonPhase)
        (Development|PrintString (Utilities|String|ToString(Float) _autoexposureminbrightness) true true "(R=0.000000,G=0.660000,B=1.000000,A=1.000000)" 9.0 "8")
        (Development|PrintString (Utilities|String|ToString(Float) _autoexposuremaxbrightness) true true "(R=0.000000,G=0.660000,B=1.000000,A=1.000000)" 2.0 "9")))))

(fn ConstructionScript
  (bind _returnvalue (Rendering|Material|CreateDynamicMaterialInstance (Variables|Default|GetSkySphereMesh) 0 "/Game/Alone/Core/World/NewSky/Material/M_Sky_Panning_Clouds2Custom.M_Sky_Panning_Clouds2Custom" "None" :!class /Script/Engine.PrimitiveComponent))
  (Variables|Default|SetSky%20material _returnvalue)
  (if (Variables|Default|GetRefresh%20material) ; Updating bool in details panel causes construction script to run again
    _
    (else
      _))
  (Variables|Default|SetRefresh%20material false)
  (Rendering|Material|SetVectorParameterValue (Variables|Default|GetSky%20material) "MoonBasicSettings" (Utilities|Struct|MakeLinearColor (/ (Variables|Default|GetMoonScale) 1e+01) (Variables|Default|GetMoonStaticRotation) (Variables|Default|GetMoonBrightness) 1.0) :!class /Script/Engine.MaterialInstanceDynamic)
  (CallFunction|RefreshMaterial)
  (CallFunction|HandleSunMoonRotation)
  (CallFunction|HandleDayNightCycle))

(fn HandleSunMoonRotation
  (bind _moonrisetime (Variables|Default|GetMoonRiseTime))
  (bind _minutesofday (Variables|Default|GetMinutesOfDay))
  (bind _dawntime (Variables|Default|GetDawnTime))
  (bind _dusktime (Variables|Default|GetDuskTime))
  (bind _sunrise0112 (LocalVariables|GetSunrise0112))
  (bind _sunset0112 (LocalVariables|GetSunset0112))
  (bind _minutesofday_2 (Variables|Default|GetMinutesOfDay))
  (bind _minutesofday_3 (Variables|Default|GetMinutesOfDay))
  (bind _moonrisetime_2 (Variables|Default|GetMoonRiseTime))
  (bind _returnvalue (Math|Float|MapRangeClamped _minutesofday _dawntime _dusktime _sunrise0112 _sunset0112))
  (bind _returnvalue_2 (+ 1.44e+03 _moonrisetime_2))
  (bind _returnvalue_3 (Math|Float|MapRangeUnclamped _minutesofday_3 0.0 _moonrisetime 1.44e+03 _returnvalue_2))
  (Utilities|FlowControl|Sequence
    (:then_0
      (if (Utilities|IsDayTime)
        (Transformation|SetWorldRotation (Variables|/Script/Engine.Actor|GetRootComponent (Variables|Default|GetDirectional%20light%20actor)) (Math|Rotator|MakeRotator 0.0 (* (Math|Curves|GetFloatValue (LocalVariables|GetAltitude) _returnvalue) -1.0) (Math|Curves|GetFloatValue (LocalVariables|GetAzimuth) _returnvalue)) false false)
        (else
          (Utilities|IsTimeBetween (Variables|Default|GetDuskTime) (+ (Variables|Default|GetDuskTime) 2e+01)
            (:true
              ;[0.15 0.15 0.15 0.5] After sunset
              (Transformation|SetWorldRotation (Variables|/Script/Engine.Actor|GetRootComponent (Variables|Default|GetDirectional%20light%20actor)) (Math|Rotator|MakeRotator 0.0 (Math|Float|MapRangeUnclamped (Variables|Default|GetMinutesOfDay) (Variables|Default|GetDuskTime) (+ (Variables|Default|GetDuskTime) 2e+01) -181.0 -2.7e+02) (Math|Curves|GetFloatValue (LocalVariables|GetAzimuth) (Variables|Default|GetMinutesOfDay))) false false))
            (:false
              (Utilities|IsTimeBetween (- (Variables|Default|GetDawnTime) 2e+01) (Variables|Default|GetDawnTime)
                (:true
                  ;[0.15 0.15 0.15 0.5] before sunrise
                  (Transformation|SetWorldRotation (Variables|/Script/Engine.Actor|GetRootComponent (Variables|Default|GetDirectional%20light%20actor)) (Math|Rotator|MakeRotator 0.0 (Math|Float|MapRangeUnclamped (Variables|Default|GetMinutesOfDay) (- (Variables|Default|GetDawnTime) 2e+01) (Variables|Default|GetDawnTime) -2.7e+02 -359.0) (Math|Curves|GetFloatValue (LocalVariables|GetAzimuth) (Variables|Default|GetMinutesOfDay))) false false))
                (:false
                  (Transformation|SetWorldRotation (Variables|/Script/Engine.Actor|GetRootComponent (Variables|Default|GetDirectional%20light%20actor)) (Math|Rotator|MakeRotator 0.0 -2.7e+02 (Math|Curves|GetFloatValue (LocalVariables|GetAzimuth) (Variables|Default|GetMinutesOfDay))) false false))))))))
    (:then_1
      (if (< (Variables|Default|GetMinutesOfDay) (Variables|Default|GetMoonRiseTime))
        (Transformation|SetWorldRotation (Variables|/Script/Engine.Actor|GetRootComponent (Variables|Default|GetMoonRef)) (Math|Rotator|MakeRotator 0.0 (* (Math|Curves|GetFloatValue (LocalVariables|GetMoonAltitude) _returnvalue_3) -1.0) (Math|Curves|GetFloatValue (LocalVariables|GetMoonAzimuth) _returnvalue_3)) false false)
        (else
          (Transformation|SetWorldRotation (Variables|/Script/Engine.Actor|GetRootComponent (Variables|Default|GetMoonRef)) (Math|Rotator|MakeRotator 0.0 (* (Math|Curves|GetFloatValue (LocalVariables|GetMoonAltitude) _minutesofday_2) -1.0) (Math|Curves|GetFloatValue (LocalVariables|GetMoonAzimuth) _minutesofday_2)) false false))))))

(fn HandleCoordinates
  (bind _month (Default|GetMonth (Variables|Default|GetGameTimeReference)))
  (Variables|Default|SetDawnTime (Math|Conversions|ToFloat(Integer) (.Value (Utilities|Map|Find (Variables|/Game/Alone/Core/World/Weather/Climate/BP_Climate.BP_Climate_C|GetSunriseTime (Variables|/Game/Alone/Core/World/Weather/BP_Weather.BP_Weather_C|GetClimateReference (Variables|Default|GetWeather%20Reference))) _month))))
  (Variables|Default|SetDuskTime (Math|Conversions|ToFloat(Integer) (.Value (Utilities|Map|Find (Variables|/Game/Alone/Core/World/Weather/Climate/BP_Climate.BP_Climate_C|GetSunsetTime (Variables|/Game/Alone/Core/World/Weather/BP_Weather.BP_Weather_C|GetClimateReference (Variables|Default|GetWeather%20Reference))) _month)))))

(fn HandleDayNightCycle
  (Development|PrintString "DayNightCycle" true true "(R=1.000000,G=0.000000,B=0.013399,A=1.000000)" 5.0 "4")
  (if (Utilities|IsDayTime)
    (Utilities|Struct|SetmembersinPostProcessSettings (Variables|/Script/Engine.PostProcessVolume|GetSettings (Variables|Default|GetPostProcessVolume)) 1e+01 14.0)
    (return)
    (else
      (Utilities|Struct|SetmembersinPostProcessSettings (Variables|/Script/Engine.PostProcessVolume|GetSettings (Variables|Default|GetPostProcessVolume)) -2.0 14.0)
      (return))))

(fn HandleMoonPhase
  (bind (_moonfullness _waning) (Default|GetMoonIllumination (Variables|Default|GetGameTimeReference)))
  (bind (_keypin _valuepin) (Utilities|Map|ForEachLoop(Map) (select _waning (LocalVariables|GetWaningList) (LocalVariables|GetWaxingList)) :!label _label)
    (:then
      (if (Math|Float|NearlyEqual(Float) _keypin _moonfullness 0.0625)
        (Rendering|Material|SetTextureParameterValue (Variables|Default|GetSky%20material) "MoonTexture" _valuepin)
        (goto _label BreakPin)))
    (:CompletedPin
      (return))))