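; Weather simulation that drives air and ocean temperature from game time and a climate object constructed at start.
; A looping timer refreshes random seasonal, multi-day and daily trends as each period ends, adding them to monthly min/max temperatures interpolated by a time-of-day curve.
; Ocean temperature moderates the result through cold/heat mitigation weights, and weighted moving averages smooth changes.
; Query functions adjust air temperature for elevation and sun exposure.
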(event Custom|Start
  (params (GameTimeReference :type BP%20Time%20Object%20Reference) (ClimateReference :type BP%20Climate%20Class%20Reference))
  (Variables|References|SetGameTimeReference GameTimeReference)
  (bind _returnvalue (Game|ConstructObjectfromClass ClimateReference))
  (Variables|References|SetClimateReference _returnvalue)
  ;[0.15 0.15 0.15 0.5] Initialize Values
  (CallFunction|UpdateWeather)
  (Variables|Default|SetInitial false)
  (Utilities|Time|SetTimerbyFunctionName 0 "UpdateWeather" 5.0 true))

(fn UpdateWeather
  (Utilities|FlowControl|Sequence
    (:then_0
      ;[0.15 0.15 0.15 0.5] Calculate seasonal trend at end of season
      (bind _month (Default|GetMonth (Variables|References|GetGameTimeReference)))
      (bind _season (Default|GetSeason (Variables|References|GetClimateReference) _month))
      (if (or (!= _season (Variables|Trends|GetSeason)) (Variables|Default|GetInitial))
        (Variables|Trends|SetSeason _season)
        (bind _weathertrend (CallFunction|CalculateTrend))
        (Variables|Trends|SetSeasonalTrend _weathertrend)))
    (:then_1
      ;[0.15 0.15 0.15 0.5] Calculate weather trend at end of current weather trend
      (if (or (> (Variables|/Game/Alone/Core/World/Time/BP_Time.BP_Time_C|GetTimePoint (Variables|References|GetGameTimeReference)) (Variables|Trends|GetLocalTrendEnd)) (Variables|Default|GetInitial))
        (bind _weathertrend_2 (CallFunction|CalculateTrend))
        (Variables|Trends|SetLocalTrend _weathertrend_2)
        (Variables|Trends|SetLocalTrendEnd (+ (* (Math|Random|RandomIntegerinRange 3 7) 1440) (Variables|/Game/Alone/Core/World/Time/BP_Time.BP_Time_C|GetTimePoint (Variables|References|GetGameTimeReference))))))
    (:then_2
      ;[0.15 0.15 0.15 0.5] Calculate daily weather
      (bind _day (Default|GetDay (Variables|References|GetGameTimeReference)))
      (if (or (> _day (Variables|Trends|GetDay)) (Variables|Default|GetInitial))
        (Variables|Trends|SetDay _day)
        ;;[0.15 0.15 0.15 0.5] Daily variation from avg temperature with consideration given to previous value
        (Variables|Trends|SetDailyTrend (Class|KismetMathLibrary|WeightedMovingAverageFloat (Math|Random|RandomFloatinRange -5.0 5.0) (Variables|Trends|GetDailyTrend) 0.5))
        ;[0.15 0.15 0.15 0.5] Calculate daily Min/Max temp
        (bind _month_2 (Default|GetMonth (Variables|References|GetGameTimeReference)))
        (bind (_avgmintemp _avgmaxtemp) (Default|GetDailyMinMax (Variables|References|GetClimateReference) _month_2))
        (if (Variables|Default|GetInitial)
          (Variables|Temperatures|SetDailyMin _avgmintemp)
          (Variables|Temperatures|SetDailyMax _avgmaxtemp)
          (else
            (Variables|Temperatures|SetDailyMin (Class|KismetMathLibrary|WeightedMovingAverageFloat _avgmintemp (Variables|Temperatures|GetDailyMin) 0.2))
            (Variables|Temperatures|SetDailyMax (Class|KismetMathLibrary|WeightedMovingAverageFloat _avgmaxtemp (Variables|Temperatures|GetDailyMax) 0.2))))
        (CallFunction|CalculateOceanTemperature :!pinned true) ; Calculate daily ocean temperature
      ))
    (:then_3
      (CallFunction|CalculateTemperature))))

(fn CalculateTrend
  (return (Math|Float|Truncate (Math|Curves|GetFloatValue (LocalVariables|GetWeatherTrendCurve) (Math|Random|RandomFloatinRange 0.0 1.0)))))

(fn CalculateTemperature
  (bind _climatereference (Variables|References|GetClimateReference))
  ;[0.15 0.15 0.15 0.5] Get temperature for current time of day
  (bind _hh_mm (Default|GetTimeOfDay (Variables|References|GetGameTimeReference)))
  (if (Variables|Default|GetInitial)
    (Variables|Temperatures|SetAirTemperature (Math|Float|Lerp (Class|KismetMathLibrary|WeightedMovingAverageFloat (+ (Math|Float|Lerp (Variables|Temperatures|GetDailyMin) (Variables|Temperatures|GetDailyMax) (Math|Curves|GetFloatValue (LocalVariables|GetDailyTemperatureCurve) _hh_mm)) (+ (Variables|Trends|GetDailyTrend) (+ (Variables|Trends|GetSeasonalTrend) (Variables|Trends|GetLocalTrend)))) (Variables|Temperatures|GetOceanTemperature) (Variables|/Game/Alone/Core/World/Weather/Climate/BP_Climate.BP_Climate_C|GetColdMitigation _climatereference)) (Class|KismetMathLibrary|WeightedMovingAverageFloat (+ (Math|Float|Lerp (Variables|Temperatures|GetDailyMin) (Variables|Temperatures|GetDailyMax) (Math|Curves|GetFloatValue (LocalVariables|GetDailyTemperatureCurve) _hh_mm)) (+ (Variables|Trends|GetDailyTrend) (+ (Variables|Trends|GetSeasonalTrend) (Variables|Trends|GetLocalTrend)))) (Variables|Temperatures|GetOceanTemperature) (Variables|/Game/Alone/Core/World/Weather/Climate/BP_Climate.BP_Climate_C|GetHeatMitigation _climatereference)) (Math|Float|Clamp(Float) (- (+ (Math|Float|Lerp (Variables|Temperatures|GetDailyMin) (Variables|Temperatures|GetDailyMax) (Math|Curves|GetFloatValue (LocalVariables|GetDailyTemperatureCurve) _hh_mm)) (+ (Variables|Trends|GetDailyTrend) (+ (Variables|Trends|GetSeasonalTrend) (Variables|Trends|GetLocalTrend)))) (Variables|Temperatures|GetOceanTemperature)))))
    (else
      ;[0.15 0.15 0.15 0.5] Set new temperature
      (Variables|Temperatures|SetAirTemperature (Class|KismetMathLibrary|WeightedMovingAverageFloat (Math|Float|Lerp (Class|KismetMathLibrary|WeightedMovingAverageFloat (+ (Math|Float|Lerp (Variables|Temperatures|GetDailyMin) (Variables|Temperatures|GetDailyMax) (Math|Curves|GetFloatValue (LocalVariables|GetDailyTemperatureCurve) _hh_mm)) (+ (Variables|Trends|GetDailyTrend) (+ (Variables|Trends|GetSeasonalTrend) (Variables|Trends|GetLocalTrend)))) (Variables|Temperatures|GetOceanTemperature) (Variables|/Game/Alone/Core/World/Weather/Climate/BP_Climate.BP_Climate_C|GetColdMitigation _climatereference)) (Class|KismetMathLibrary|WeightedMovingAverageFloat (+ (Math|Float|Lerp (Variables|Temperatures|GetDailyMin) (Variables|Temperatures|GetDailyMax) (Math|Curves|GetFloatValue (LocalVariables|GetDailyTemperatureCurve) _hh_mm)) (+ (Variables|Trends|GetDailyTrend) (+ (Variables|Trends|GetSeasonalTrend) (Variables|Trends|GetLocalTrend)))) (Variables|Temperatures|GetOceanTemperature) (Variables|/Game/Alone/Core/World/Weather/Climate/BP_Climate.BP_Climate_C|GetHeatMitigation _climatereference)) (Math|Float|Clamp(Float) (- (+ (Math|Float|Lerp (Variables|Temperatures|GetDailyMin) (Variables|Temperatures|GetDailyMax) (Math|Curves|GetFloatValue (LocalVariables|GetDailyTemperatureCurve) _hh_mm)) (+ (Variables|Trends|GetDailyTrend) (+ (Variables|Trends|GetSeasonalTrend) (Variables|Trends|GetLocalTrend)))) (Variables|Temperatures|GetOceanTemperature)))) (Variables|Temperatures|GetAirTemperature) 0.2)))))

(fn CalculateOceanTemperature
  (bind _month (Default|GetMonth (Variables|References|GetGameTimeReference)))
  (bind _oceantemperature (Default|GetOceanTemp (Variables|References|GetClimateReference) _month))
  (if (Variables|Default|GetInitial)
    (Variables|Temperatures|SetOceanTemperature (+ _oceantemperature (Math|Random|RandomFloatinRange -2.0 2.0)))
    (else
      (Variables|Temperatures|SetOceanTemperature (Class|KismetMathLibrary|WeightedMovingAverageFloat (+ _oceantemperature (Math|Random|RandomFloatinRange -2.0 2.0)) (Variables|Temperatures|GetOceanTemperature) 0.75)))))

(fn TemperatureatElevation
  (params (Elevation :type Float%20%28double-precision%29))
  (return (- (- (Math|Float|Clamp(Float) (+ (Variables|Temperatures|GetAirTemperature) 5e+01) 0.0 1e+02) (/ (/ Elevation 1e+02) 1e+02)) 5e+01)))

(fn FeelsLike
  (params (Elevation :type Float%20%28double-precision%29) (InShade :type Boolean))
  (bind _temperature (CallFunction|TemperatureatElevation Elevation))
  (if InShade
    (return _temperature)
    (else
      (return (+ _temperature 5.0)))))