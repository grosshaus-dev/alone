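; BP_Climate is a climate data Blueprint for the weather system that answers per-month season and temperature queries.
; GetSeason tests the month against summer, fall, winter and spring collections in turn and returns the matching season.
; GetDailyMinMax and GetOceanTemp look up average minimum and maximum temperatures and average ocean temperature in maps keyed by month.
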(fn GetSeason
  (params (Month :type Integer))
  (if (Utilities|Array|ContainsItem (Variables|Default|GetSeasonSummer) Month)
    (return 0)
    (elif (Utilities|Array|ContainsItem (Variables|Default|GetSeasonFall) Month)
      (return 1)
      (elif (Utilities|Array|ContainsItem (Variables|Default|GetSeasonWinter) Month)
        (return 2)
        (elif (Utilities|Array|ContainsItem (Variables|Default|GetSeasonSpring) Month)
          (return 3))))))

(fn GetDailyMinMax
  (params (Month :type Integer))
  (return (.Value (Utilities|Map|Find (Variables|Default|GetAvgMinTemp) Month)) (.Value (Utilities|Map|Find (Variables|Default|GetAvgMaxTemp) Month))))

(fn GetOceanTemp
  (params (Month :type Integer))
  (return (.Value (Utilities|Map|Find (Variables|Default|GetAvgOceanTemp) Month))))