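; BP_Weather simulates air temperature from in-game time and a climate object it constructs on Start.
; A looping five-second timer re-rolls a seasonal trend on season change and a shorter trend after a randomized number of days, both via a random-sampled curve.
; Temperature blends monthly min/max averages along a daily curve, then adds both trends and random noise.
; The noise re-rolls every update, though an inline note says once per day/night cycle.
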(event Custom|Start
  (params (GameTimeReference :type BP%20Time%20Object%20Reference) (ClimateReference :type BP%20Climate%20Class%20Reference))
  (Variables|References|SetGameTimeReference GameTimeReference)
  (bind _returnvalue (Game|ConstructObjectfromClass ClimateReference))
  (Variables|References|SetClimateReference _returnvalue)
  (Utilities|Time|SetTimerbyFunctionName 0 "UpdateWeather" 5.0 true))

(fn UpdateWeather
  (Utilities|FlowControl|Sequence
    (:then_0
      ;[0.15 0.15 0.15 0.5] Calculate seasonal trend at end of season
      (bind _month (Default|GetMonth (Variables|References|GetGameTimeReference)))
      (bind _season (Default|GetSeason (Variables|References|GetClimateReference) _month))
      (if (!= _season (Variables|Trends|GetCurrentSeason))
        (Variables|Trends|SetCurrentSeason _season)
        (bind _weathertrend (CallFunction|CalculateTrend))
        (Variables|Trends|SetCurrentSeasonTrend _weathertrend)))
    (:then_1
      ;[0.15 0.15 0.15 0.5] Calculate weather trend at end of current weather trend
      (if (> (Variables|/Game/Alone/Core/World/Time/BP_Time.BP_Time_C|GetTimePoint (Variables|References|GetGameTimeReference)) (Variables|Trends|GetTrendEndTimePoint))
        (bind _weathertrend_2 (CallFunction|CalculateTrend))
        (Variables|Trends|SetTrend _weathertrend_2)
        (Variables|Trends|SetTrendEndTimePoint (+ (* (+ (Variables|Trends|GetAvgTrendLength) (Math|Random|RandomIntegerinRange -2 2)) 1440) (Variables|/Game/Alone/Core/World/Time/BP_Time.BP_Time_C|GetTimePoint (Variables|References|GetGameTimeReference))))))
    (:then_2
      (CallFunction|CalculateTemperature))))

(fn CalculateTrend
  (return (Math|Float|Truncate (Math|Curves|GetFloatValue (LocalVariables|GetWeatherTrendCurve) (Math|Random|RandomFloatinRange 0.0 1.0)))))

(fn CalculateTemperature
  (bind _hh_mm (Default|GetTimeOfDay (Variables|References|GetGameTimeReference)))
  (bind _month (Default|GetMonth (Variables|References|GetGameTimeReference)))
  (bind (_avgmintemp _avgmaxtemp) (Default|GetDailyMinMax (Variables|References|GetClimateReference) _month))
  (Variables|Default|SetAirTemperature (+ (Math|Float|Lerp _avgmintemp _avgmaxtemp (Math|Curves|GetFloatValue (LocalVariables|GetDailyTemperatureCurve) _hh_mm)) (+ (Math|Random|RandomFloatinRange -3.0 3.0) (+ (Variables|Trends|GetCurrentSeasonTrend) (Variables|Trends|GetTrend))))))