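; BP_Time is the game clock, counting scaled game minutes in a single TimePoint that a pausable looping timer increments and PassTime can advance.
; Day, month and time of day all derive from TimePoint, with months looked up through a Days map over a 365-day year.
; Moon illumination and semidiurnal tide sample a shared wave curve on modulo cycles, and moon fullness widens the tide range within a supplied HAT.
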(event Custom|Start
  ;[1 1 1] Calls tick on an interval to increment time point (SCALED GAME TIME)
  (Utilities|Time|SetTimerbyFunctionName 0 "Tick" (Variables|Default|GetTickIntervalInSeconds) true))

(event Custom|Pause
  ;[1 1 1] Pause tick
  (Class|KismetSystemLibrary|PauseTimer 0 "Tick"))

(event Custom|Unpause
  ;[1 1 1] Unpause tick
  (Class|KismetSystemLibrary|UnPauseTimer 0 "Tick"))

(fn Tick
  (Math|Integer|IncrementInt (Variables|Default|GetTimePoint)))

(fn PassTime
  (params (TimePassed :type Integer))
  (Variables|Default|SetTimePoint (+ TimePassed (Variables|Default|GetTimePoint))))

(fn GetMoonIllumination
  (bind _timepoint (Variables|Default|GetTimePoint))
  (bind _returnvalue (Math|Integer|%(Integer) _timepoint 42480))
  (bind _returnvalue_2 (Math|Conversions|ToFloat(Integer) _returnvalue))
  (bind _returnvalue_3 (/ _returnvalue_2 4.248e+04))
  (return (Math|Curves|GetFloatValue (Variables|Default|GetStandardWaveCurve) _returnvalue_3) (> _returnvalue_3 0.5)))

(fn GetSemidiurnalTideFloodPercent
  (return (Math|Curves|GetFloatValue (Variables|Default|GetStandardWaveCurve) (/ (Math|Conversions|ToFloat(Integer) (Math|Integer|%(Integer) (Variables|Default|GetTimePoint) 780)) 7.8e+02))))

(fn GetTideLevel
  (params (HAT :type Float%20%28double-precision%29))
  ;[0.15 0.15 0.15 0.5] Calculate the moon's effect on the tide
  (bind _moonfullness (CallFunction|GetMoonIllumination))
  (bind _tidefloodpercent (CallFunction|GetSemidiurnalTideFloodPercent)) ; Can be expanded in case Diurnal or Mixed Semidiurnal tides need to be supported.
  (return (+ (* _tidefloodpercent (- (+ (* HAT 0.8) (* _moonfullness (* HAT 0.2))) (- (* HAT 0.2) (* _moonfullness (* HAT 0.2))))) (- (* HAT 0.2) (* _moonfullness (* HAT 0.2))))))

(fn GetMonth
  (bind _days (Variables|Default|GetDays))
  (bind _value (Utilities|Map|GetKeyValueByIndex _days 2))
  (bind _value_2 (Utilities|Map|GetKeyValueByIndex _days 3))
  (bind _value_3 (Utilities|Map|GetKeyValueByIndex _days 4))
  (bind _value_4 (Utilities|Map|GetKeyValueByIndex _days 5))
  (bind _value_5 (Utilities|Map|GetKeyValueByIndex _days 6))
  (bind _value_6 (Utilities|Map|GetKeyValueByIndex _days 7))
  (bind _value_7 (Utilities|Map|GetKeyValueByIndex _days 8))
  (bind _value_8 (Utilities|Map|GetKeyValueByIndex _days 9))
  (bind _value_9 (Utilities|Map|GetKeyValueByIndex _days 10))
  (bind _value_10 (Utilities|Map|GetKeyValueByIndex _days 11))
  (bind _value_11 (Utilities|Map|GetKeyValueByIndex _days 1))
  (bind _day (CallFunction|GetDay))
  (if (Math|Integer|InRange(Integer) (Math|Integer|%(Integer) _day 365) 1 _value_11)
    (return 1)
    (elif (Math|Integer|InRange(Integer) (Math|Integer|%(Integer) _day 365) _value_11 _value false)
      (return 2)
      (elif (Math|Integer|InRange(Integer) (Math|Integer|%(Integer) _day 365) _value _value_2 false)
        (return 3)
        (elif (Math|Integer|InRange(Integer) (Math|Integer|%(Integer) _day 365) _value_2 _value_3 false)
          (return 4)
          (elif (Math|Integer|InRange(Integer) (Math|Integer|%(Integer) _day 365) _value_3 _value_4 false)
            (return 5)
            (elif (Math|Integer|InRange(Integer) (Math|Integer|%(Integer) _day 365) _value_4 _value_5 false)
              (return 6)
              (elif (Math|Integer|InRange(Integer) (Math|Integer|%(Integer) _day 365) _value_5 _value_6 false)
                (return 7)
                (elif (Math|Integer|InRange(Integer) (Math|Integer|%(Integer) _day 365) _value_6 _value_7 false)
                  (return 8)
                  (elif (Math|Integer|InRange(Integer) (Math|Integer|%(Integer) _day 365) _value_7 _value_8 false)
                    (return 9)
                    (elif (Math|Integer|InRange(Integer) (Math|Integer|%(Integer) _day 365) _value_8 _value_9 false)
                      (return 10)
                      (elif (Math|Integer|InRange(Integer) (Math|Integer|%(Integer) _day 365) _value_9 _value_10 false)
                        (return 11)
                        (elif (Math|Integer|InRange(Integer) (Math|Integer|%(Integer) _day 365) _value_10 (.Value (Utilities|Map|GetKeyValueByIndex _days 12)) false)
                          (return 12)
                          (else
                            (return 0)))))))))))))))

(fn GetTimeOfDay
  (bind _timepoint (Variables|Default|GetTimePoint))
  (bind _returnvalue (Math|Integer|%(Integer) _timepoint 1440))
  (bind _returnvalue_2 (Math|Integer|%(Integer) _returnvalue 60))
  (bind _returnvalue_3 (/ _returnvalue 60))
  (return _returnvalue_3 _returnvalue_2 (+ (Math|Conversions|ToFloat(Integer) _returnvalue_3) (/ (Math|Conversions|ToFloat(Integer) _returnvalue_2) 1e+02))))

(fn GetDay
  (return (+ (/ (Variables|Default|GetTimePoint) 1440) 1)))