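; BP_AloneFlammableObject is an actor that can ignite, burn over time and spread fire to nearby objects.
; Ignite checks strength against a threshold, then swaps to a burning material, shows a light and starts a looping timer.
; The timer advances burn time and lowers Condition until the object is destroyed or left charred.
; Fire spreads through delayed Ignite messages to actors overlapping BurnRadius, and active objects self-ignite after BeginPlay.
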(event OnComponentBeginOverlap(BurnRadius)
  (params (OverlappedComponent :type Primitive%20Component%20Object%20Reference) (OtherActor :type Actor%20Object%20Reference) (OtherComp :type Primitive%20Component%20Object%20Reference) (OtherBodyIndex :type Integer) (bFromSweep :type Boolean) (SweepResult :type Hit%20Result%20Structure%20%28by%20ref%29))
  (Utilities|FlowControl|Delay 2.0)
  (if (Variables|Default|GetIsBurning)
    (Class|BPIFlammable|Ignite(Message) OtherActor 3)))

(event Custom|Event%20Burning
  (if (>= (Variables|Default|GetBurnTime) (Variables|Default|GetBurnValue))
    (Utilities|Time|PauseTimerbyHandle (stale EventIgnite _returnvalue))
    (Rendering|SetVisibility (Variables|Default|GetFireLight) false false)
    (if (Variables|Default|GetBurnDown)
      (Actor|DestroyActor)
      (else
        (Rendering|Material|SetMaterial (Variables|Default|GetObject) 0 (Variables|Default|GetCharred))
        (Variables|Default|SetIsCharred true)
        (bind _output_get (Variables|Default|SetIsBurning false))
        (Variables|Default|Setactive _output_get)))
    (else
      (bind _output_get_2 (Variables|Default|SetBurnTime (+ (Variables|Default|GetBurnTime) (Variables|Default|GetTick))))
      (Variables|Default|SetCondition (- 1e+02 (* (/ 1e+02 (Variables|Default|GetBurnValue)) _output_get_2))))))

(event Collision|EventActorBeginOverlap
  (params (OtherActor :type Actor%20Object%20Reference)))

(event EventTick
  (params (DeltaSeconds :type Float%20%28single-precision%29)))

(event EventIgnite
  (params (IgnitionStrength :type Integer))
  (if (Math|Boolean|ANDBoolean (>= IgnitionStrength (Variables|Default|GetIgnitionThreshold)) (!= (Variables|Default|GetIsCharred) true) (!= (Variables|Default|GetIsBurning) true))
    (bind _output_get (Variables|Default|SetIsBurning true))
    (Variables|Default|Setactive _output_get)
    (Rendering|Material|SetMaterial (Variables|Default|GetObject) 0 (Variables|Default|GetBurning))
    (Rendering|SetVisibility (Variables|Default|GetFireLight) true false)
    (bind _returnvalue (Utilities|Time|SetTimerbyEvent (delegate Custom|Event%20Burning) (Variables|Default|GetTick) true true))
    (Development|PrintString "search for near objects")
    (Utilities|FlowControl|Delay 2.0)
    (for _array_element (Collision|GetOverlappingActors (Variables|Default|GetBurnRadius) "BP_AloneFlammableObject_C" :!class /Script/Engine.PrimitiveComponent)
      (Class|BPIFlammable|Ignite(Message) _array_element 3))))

(event EventBeginPlay
  ;[0.15 0.15 0.15 0.5] BurnTime-BurnValue/100*Condition
  (bind _output_get (Variables|Default|SetBurnTime (- (Variables|Default|GetBurnValue) (* (/ (Variables|Default|GetBurnValue) 1e+02) (Variables|Default|GetCondition)))))
  (if (Variables|Default|Getactive)
    (Development|PrintString (Utilities|String|ToString(Float) _output_get) true true "(R=1.000000,G=0.000000,B=0.347263,A=1.000000)")
    (Utilities|FlowControl|Delay 3.0)
    (CallFunction|Ignite (Variables|Default|GetIgnitionThreshold))))

(fn ConstructionScript)