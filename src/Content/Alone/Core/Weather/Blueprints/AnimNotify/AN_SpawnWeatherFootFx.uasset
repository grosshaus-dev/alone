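; Anim notify that spawns weather-dependent Niagara footstep effects when a character's foot lands.
; When its trace check passes, it picks the bone for the landing foot and traces down from it against WorldStatic objects.
; Snowy weather spawns a left or right foot effect at the hit, rotated to the owning actor.
; Rainy weather spawns a splash only when the hit surface type is Puddle.
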(fn ReceivedNotify
  (params (MeshComp :type Skeletal%20Mesh%20Component%20Object%20Reference) (Animation :type Anim%20Sequence%20Base%20Object%20Reference) (EventReference :type Anim%20Notify%20Event%20Reference%20Structure%20%28by%20ref%29))
  (bind _returnvalue (Utilities|ShouldDoLineTrace))
  (if _returnvalue
    (switch Utilities|FlowControl|Switch|SwitchonEFootType (Variables|Default|GetCurrentLandingFoot)
      (:NewEnumerator0
        (LocalVariables|SetCurrentLandingBoneName "foot_l"))
      (:NewEnumerator1
        (LocalVariables|SetCurrentLandingBoneName "foot_r")))
    (bind _outhit (Collision|LineTraceForObjects (Transformation|GetSocketLocation MeshComp (LocalVariables|GetCurrentLandingBoneName)) (+ (Transformation|GetSocketLocation MeshComp (LocalVariables|GetCurrentLandingBoneName)) (* (* (Math|Vector|GetUpVector MeshComp) -1.0) 1e+02)) (Utilities|Array|MakeArray "ObjectTypeQuery1") false 0 "None"))
    (LocalVariables|SetCurrentSurfaceHitResult _outhit)
    (Utilities|GetCurrentWeatherType
      (:Snowy
        (Niagara|SpawnSystematLocation (select (Utilities|String|Contains (Utilities|String|ToString(Name) (LocalVariables|GetCurrentLandingBoneName)) "_l") "/Game/Alone/Core/Weather/Niagara/Footprints/NS_LeftFoot.NS_LeftFoot" "/Game/Alone/Core/Weather/Niagara/Footprints/NS_RightFoot.NS_RightFoot") (.Location (Collision|BreakHitResult (LocalVariables|GetCurrentSurfaceHitResult))) (Transformation|GetActorRotation (Components|GetOwner MeshComp)))
        (return false))
      (:Rainy
        (switch Utilities|FlowControl|Switch|SwitchonEPhysicalSurface (Collision|GetSurfaceType (LocalVariables|GetCurrentSurfaceHitResult))
          (:SurfaceType1
            (Niagara|SpawnSystematLocation "/Game/Alone/Core/Weather/Niagara/Rain/NS_PuddleSplash.NS_PuddleSplash" (.Location (Collision|BreakHitResult (LocalVariables|GetCurrentSurfaceHitResult))))))))))