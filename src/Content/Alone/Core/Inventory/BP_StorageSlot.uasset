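; BP_StorageSlot is an inventory slot actor that tells its container when the item it holds leaves.
; On spawn it hides its Sphere if its X scale is 0.1, marking a used slot.
; When its RemovableItem ends overlap with Sphere1, after the container is ready to close and the item's move has ended, it calls RemoveItem on the container and destroys itself.
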(event OnComponentEndOverlap(Sphere1)
  (params (OverlappedComponent :type Primitive%20Component%20Object%20Reference) (OtherActor :type Actor%20Object%20Reference) (OtherComp :type Primitive%20Component%20Object%20Reference) (OtherBodyIndex :type Integer))
  (bind _containerref (Variables|Default|GetContainerRef))
  ;[0.15 0.15 0.15 0.5] Remove full slot an send message back to container
  (bind _asbp_alone_world_object (Utilities|Casting|CastToBP_AloneWorldObject OtherActor))
  (Utilities|IsValid (Variables|Default|GetContainerRef)
    (:Is%20Valid
      (if (Math|Boolean|ANDBoolean (== OtherActor (Variables|Default|GetRemovable%20Item)) (!= self (Variables|Default|GetRemovable%20Item)) (Variables|/Game/Alone/Models/Items/Containers/BP_Container.BP_Container_C|GetReadyToClose (Variables|Default|GetContainerRef)) (Variables|/Game/Alone/Core/BP_AloneWorldObject.BP_AloneWorldObject_C|Getend%20Move _asbp_alone_world_object))
        (Variables|Default|SetRemovable%20Item self)
        (Development|PrintString "end overlap")
        (Utilities|IsValid _containerref
          (:Is%20Valid
            (Default|RemoveItem _containerref _asbp_alone_world_object)
            (Actor|DestroyActor)))))))

(event EventBeginPlay
  ;[0.15 0.15 0.15 0.5] Used slots are invisible at spawn
  (if (== (.x (Transformation|GetActorScale3D)) 0.1)
    (Rendering|SetVisibility (Variables|Default|GetSphere) false false)))

(fn ConstructionScript)