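; BP_EmptyCarrySlot is an empty inventory carry slot that accepts a world object the player is holding.
; When the grabbed object enters its box, the sphere turns dark glass and a looping timer polls until the player's grabbed item changes.
; It then stops the object's physics, moves it to the sphere and adds it to the player's inventory component.
; Leaving the box while still grabbed restores the glass and cancels polling.
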(event OnComponentBeginOverlap(Box)
  (params (OverlappedComponent :type Primitive%20Component%20Object%20Reference) (OtherActor :type Actor%20Object%20Reference) (OtherComp :type Primitive%20Component%20Object%20Reference) (OtherBodyIndex :type Integer) (bFromSweep :type Boolean) (SweepResult :type Hit%20Result%20Structure%20%28by%20ref%29))
  (bind _asalone_player_character (Utilities|Casting|CastToAlonePlayerCharacter (Game|GetPlayerCharacter 0)))
  (if (and (== (Variables|/Game/Alone/Core/PlayerCharacter/AlonePlayerCharacter.AlonePlayerCharacter_C|GetItemGrabbing _asalone_player_character) OtherActor) (!= (Utilities|GetClass OtherComp) "/Script/Engine.SphereComponent"))
    (Rendering|Material|SetMaterial (Variables|Default|GetSphere_0) 0 "/Game/Alone/Materials/Glass/MI_Glass_Dark.MI_Glass_Dark")
    (bind _asbp_alone_world_object (Utilities|Casting|CastToBP_AloneWorldObject OtherActor))
    (Variables|Default|SetNewItem _asbp_alone_world_object)
    (bind _returnvalue (Utilities|Time|SetTimerbyEvent (delegate Custom|End%20Of%20Grabbing?) 0.2 true true))
    (Variables|Default|SetQuestion _returnvalue)))

(event OnComponentEndOverlap(Box)
  (params (OverlappedComponent :type Primitive%20Component%20Object%20Reference) (OtherActor :type Actor%20Object%20Reference) (OtherComp :type Primitive%20Component%20Object%20Reference) (OtherBodyIndex :type Integer))
  (bind _asalone_player_character (Utilities|Casting|CastToAlonePlayerCharacter (Game|GetPlayerCharacter 0)))
  (if (== (Variables|/Game/Alone/Core/PlayerCharacter/AlonePlayerCharacter.AlonePlayerCharacter_C|GetItemGrabbing _asalone_player_character) OtherActor)
    (Rendering|Material|SetMaterial (Variables|Default|GetSphere_0) 0 "/Game/Alone/Materials/M_Glass.M_Glass")
    (Variables|Default|SetNewItem 0)
    (Utilities|Time|ClearandInvalidateTimerbyHandle (Variables|Default|GetQuestion))))

(event Custom|End%20Of%20Grabbing?
  (bind _asalone_player_character (Utilities|Casting|CastToAlonePlayerCharacter (Game|GetPlayerCharacter 0)))
  (if (and (Utilities|IsValid (Variables|Default|GetNewItem)) (!= (Variables|Default|GetNewItem) (Variables|/Game/Alone/Core/PlayerCharacter/AlonePlayerCharacter.AlonePlayerCharacter_C|GetItemGrabbing _asalone_player_character)))
    (Utilities|Time|ClearandInvalidateTimerbyHandle (Variables|Default|GetQuestion))
    (Physics|SetSimulatePhysics (Variables|/Game/Alone/Core/BP_AloneWorldObject.BP_AloneWorldObject_C|GetRootStaticMesh (Variables|Default|GetNewItem)) false)
    (Transformation|SetActorLocation (Variables|Default|GetNewItem) (Transformation|GetWorldLocation (Variables|Default|GetSphere_0)) true false)
    (Collision|SetActorEnableCollision true)
    (bind _asalone_player_character_2 (Utilities|Casting|CastToAlonePlayerCharacter (Game|GetPlayerCharacter 0)))
    (Default|AddItem (Variables|/Game/Alone/Core/PlayerCharacter/AlonePlayerCharacter.AlonePlayerCharacter_C|GetAC_Inventory _asalone_player_character_2) (Variables|Default|GetCarrySlotID) (Variables|Default|GetNewItem) self)
    (Variables|Default|SetNewItem 0)))

(event EventBeginPlay)

(fn ConstructionScript)