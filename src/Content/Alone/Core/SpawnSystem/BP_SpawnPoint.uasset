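; Spawn point pickup, shown as a message in a bottle, that the player takes to unlock a named spawn point and its region.
; On BeginPlay it polls until the player is ready, then restores its broken-bottle look if the global save already lists it.
; Interacting records the unlock, notifies, awards more XP for a new region than a known one, saves and breaks the bottle.
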(event EventInteract
  (bind _region (Variables|Default|GetRegion))
  ;[0.15 0.15 0.15 0.5] Unlock spawn point
  (if (not (Variables|Default|GetUnlocked))
    (bind _asalone_player_character (Utilities|Casting|CastToAlonePlayerCharacter (Game|GetPlayerCharacter 0)))
    (Utilities|Set|Add (Variables|/Game/Alone/Core/Save/Save_AloneGlobal.Save_AloneGlobal_C|GetGoodHopeUnlockedSpawnPoints (Variables|/Game/Alone/Core/PlayerCharacter/AlonePlayerCharacter.AlonePlayerCharacter_C|GetGlobalSaveObject _asalone_player_character)) (Variables|Default|GetName))
    (if (Utilities|Set|Contains (Variables|/Game/Alone/Core/Save/Save_AloneGlobal.Save_AloneGlobal_C|GetGoodHopeUnlockedRegions (Variables|/Game/Alone/Core/PlayerCharacter/AlonePlayerCharacter.AlonePlayerCharacter_C|GetGlobalSaveObject _asalone_player_character)) _region)
      (CallFunction|ALNNotify "Unlocked Spawn Point" (Utilities|Text|ToText(String) (Utilities|String|Append (Utilities|String|EnumtoString (Variables|Default|GetRegion)) ": " (Utilities|String|ToString(Name) (Variables|Default|GetName)))))
      ;;[0.15 0.15 0.15 0.5] Gain XP for unlocking spawn point
      (Variables|/Game/Alone/Core/Save/Save_AloneGlobal.Save_AloneGlobal_C|SetXP (Variables|/Game/Alone/Core/PlayerCharacter/AlonePlayerCharacter.AlonePlayerCharacter_C|GetGlobalSaveObject _asalone_player_character) (+ (Variables|/Game/Alone/Core/Save/Save_AloneGlobal.Save_AloneGlobal_C|GetXP (Variables|/Game/Alone/Core/PlayerCharacter/AlonePlayerCharacter.AlonePlayerCharacter_C|GetGlobalSaveObject _asalone_player_character)) 10))
      (else
        (Utilities|Set|Add (Variables|/Game/Alone/Core/Save/Save_AloneGlobal.Save_AloneGlobal_C|GetGoodHopeUnlockedRegions (Variables|/Game/Alone/Core/PlayerCharacter/AlonePlayerCharacter.AlonePlayerCharacter_C|GetGlobalSaveObject _asalone_player_character)) _region)
        (CallFunction|ALNNotify "Unlocked Region" (Utilities|Text|ToText(String) (Utilities|String|EnumtoString (Variables|Default|GetRegion))))
        ;;[0.15 0.15 0.15 0.5] Gain XP for unlocking new region
        (Variables|/Game/Alone/Core/Save/Save_AloneGlobal.Save_AloneGlobal_C|SetXP (Variables|/Game/Alone/Core/PlayerCharacter/AlonePlayerCharacter.AlonePlayerCharacter_C|GetGlobalSaveObject _asalone_player_character) (+ (Variables|/Game/Alone/Core/Save/Save_AloneGlobal.Save_AloneGlobal_C|GetXP (Variables|/Game/Alone/Core/PlayerCharacter/AlonePlayerCharacter.AlonePlayerCharacter_C|GetGlobalSaveObject _asalone_player_character)) 100))))
    (Default|SaveGame _asalone_player_character)
    (Variables|Default|SetUnlocked true)
    (Components|DestroyComponent (Variables|Default|GetMessage))
    (Components|StaticMesh|SetStaticMesh (Variables|Default|GetBottle) "/Game/Alone/Models/Items/Bottles/SM_Bottle_Broken_01.SM_Bottle_Broken_01")))

(event EventBeginPlay
  ;[0.15 0.15 0.15 0.5] Check if spawn point is already unlocked
  (bind _asalone_player_character (Utilities|Casting|CastToAlonePlayerCharacter (Game|GetPlayerCharacter 0)))
  ;;[0.15 0.15 0.15 0.5] Wair for player character to be ready
  (if (Variables|/Game/Alone/Core/PlayerCharacter/AlonePlayerCharacter.AlonePlayerCharacter_C|GetReady _asalone_player_character) :!label _label
    (bind _output_get (Variables|Default|SetUnlocked (Utilities|Set|Contains (Variables|/Game/Alone/Core/Save/Save_AloneGlobal.Save_AloneGlobal_C|GetGoodHopeUnlockedSpawnPoints (Variables|/Game/Alone/Core/PlayerCharacter/AlonePlayerCharacter.AlonePlayerCharacter_C|GetGlobalSaveObject _asalone_player_character)) (Variables|Default|GetName))))
    (if _output_get
      (Components|DestroyComponent (Variables|Default|GetMessage))
      (Components|StaticMesh|SetStaticMesh (Variables|Default|GetBottle) "/Game/Alone/Models/Items/Bottles/SM_Bottle_Broken_01.SM_Bottle_Broken_01"))
    (else
      (Utilities|FlowControl|Delay 0.2)
      (goto _label))))

(fn ConstructionScript)

(fn GetAltInteractionText
  (return ""))

(fn GetInteractionText
  (if (Variables|Default|GetUnlocked)
    (return "")
    (else
      (return "Take"))))