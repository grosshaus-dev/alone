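; BP_Time is the game clock, keeping scaled game time as an incrementing TimePoint counter.
; Start sets a looping timer that calls its Tick function every TickIntervalInSeconds, adding one to TimePoint each call.
; Pause and Unpause suspend and resume that timer, while PassTime jumps the clock forward by adding a given amount to TimePoint.
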(event Custom|Start
  ;[1 1 1] Calls tick on an interval to increment time point (SCALED GAME TIME)
  (Utilities|Time|SetTimerbyFunctionName 0 "Tick" (Variables|Default|GetTickIntervalInSeconds) true))

(event Custom|Pause
  ;[1 1 1] Pause tick
  (Class|KismetSystemLibrary|PauseTimer 0 "Tick"))

(event Custom|Unpause
  ;[1 1 1] Unpause tick
  (Class|KismetSystemLibrary|UnPauseTimer 0 "Tick"))

(fn Tick
  (Math|Integer|IncrementInt (Variables|Default|GetTimePoint)))

(fn PassTime
  (params (TimePassed :type Integer))
  (Variables|Default|SetTimePoint (+ TimePassed (Variables|Default|GetTimePoint))))