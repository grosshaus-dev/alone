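; AC_Burnable is a component that lets an object burn for a set duration, then stay permanently burnt down.
; The Burning event swaps the referenced mesh to its burning version, shows the light and disables shadow casting.
; After a Delay, SetBurnt restores the normal mesh and shadow, hides the light, applies a burnt wood material and blocks re-ignition.
; Both interaction text getters return empty strings.
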(event Custom|Burning
  (if (not (Variables|Default|GetIs%20Burnt%20Down))
    (CallFunction|Burn (Variables|Default|GetBurning%20Mesh))
    (Utilities|FlowControl|Delay (Variables|Default|GetDuration))
    (CallFunction|SetBurnt (Variables|Default|GetNormal%20Mesh))))

(event EventTick
  (params (DeltaSeconds :type Float%20%28single-precision%29)))

(fn Burn
  (params (Burning%20Mesh :type Static%20Mesh%20Object%20Reference))
  (Utilities|FlowControl|Sequence
    (:then_0
      (if (not (Variables|Default|GetIs%20burning))
        (Variables|Default|SetIs%20burning true)
        (Components|StaticMesh|SetStaticMesh (Variables|Default|GetMesh%20ref) Burning%20Mesh)
        (Rendering|SetVisibility (Variables|Default|GetLight%20ref) true false)
        (Rendering|SetCastShadow (Variables|Default|GetMesh%20ref) false)))))

(fn SetBurnt
  (params (Normal%20Mesh :type Static%20Mesh%20Object%20Reference))
  (Variables|Default|SetIs%20burning false)
  (Components|StaticMesh|SetStaticMesh (Variables|Default|GetMesh%20ref) Normal%20Mesh)
  (Rendering|SetVisibility (Variables|Default|GetLight%20ref) false false)
  (Rendering|SetCastShadow (Variables|Default|GetMesh%20ref) true)
  (Rendering|Material|SetMaterial (Variables|Default|GetMesh%20ref) 0 "/Game/Alone/Materials/Plant/MI_WoodLightBurndDown.MI_WoodLightBurndDown")
  (Variables|Default|SetIs%20Burnt%20Down true))

(fn GetAltInteractionText
  (return ""))

(fn GetInteractionText
  (return ""))