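; BP_Controller_Game is the in-game player controller that sets up Enhanced Input, game-only input and the HUD on begin play.
; Pause halts the player's game-time reference and the game, clears all widgets, then opens the pause menu with UI-only input.
; Info and Help actions toggle debug and help panels by searching for existing widgets.
; A dev trigger sends a spawn tick message to every actor implementing the spawner interface.
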(event Input|EnhancedActionEvents|EnhancedInputActionIA_Pause
  (params (ActionValue :type Boolean) (ElapsedSeconds :type Float%20%28double-precision%29) (TriggeredSeconds :type Float%20%28double-precision%29) (InputAction :type Input%20Action%20Object%20Reference :default "/Game/Alone/Core/Input/Actions/IA_Pause.IA_Pause"))
  ;[1 1 1] Pause Game
  (:Triggered
    ;;[1 1 1] Pause game time tick
    (bind _asalone_player_character (Utilities|Casting|CastToAlonePlayerCharacter (Game|GetPlayerCharacter 0)))
    (Default|Pause (Variables|/Game/Alone/Core/PlayerCharacter/AlonePlayerCharacter.AlonePlayerCharacter_C|GetGameTimeReference _asalone_player_character))
    (Game|SetGamePaused true)
    (Viewport|RemoveAllWidgets)
    (bind _returnvalue (UserInterface|CreateWidget "/Game/Alone/UI/W_Menu_Pause.W_Menu_Pause_C"))
    (UserInterface|Viewport|AddtoViewport _returnvalue 0)
    (Variables|Default|SetbShowMouseCursor true)
    (Input|SetInputModeUIOnly (Game|GetPlayerController 0) _returnvalue "DoNotLock" true)))

(event Input|EnhancedActionEvents|EnhancedInputActionIA_Info
  (params (ActionValue :type Boolean) (ElapsedSeconds :type Float%20%28double-precision%29) (TriggeredSeconds :type Float%20%28double-precision%29) (InputAction :type Input%20Action%20Object%20Reference :default "/Game/Alone/Core/Input/Actions/IA_Info.IA_Info"))
  ;[1 1 1] Show/hide info panel
  (:Triggered
    (bind _foundwidgets (Widget|GetAllWidgetsOfClass "/Game/Alone/UI/HUD/W_Panel_Debug.W_Panel_Debug_C" true))
    (if (Utilities|Array|IsEmpty _foundwidgets)
      (bind _returnvalue (UserInterface|CreateWidget "/Game/Alone/UI/HUD/W_Panel_Debug.W_Panel_Debug_C"))
      (UserInterface|Viewport|AddtoViewport _returnvalue 0)
      (Variables|Default|SetbShowMouseCursor true)
      (else
        (for _array_element _foundwidgets
          (Widget|RemovefromParent _array_element)
          (Variables|Default|SetbShowMouseCursor false))))))

(event Input|EnhancedActionEvents|EnhancedInputActionIA_Help
  (params (ActionValue :type Boolean) (ElapsedSeconds :type Float%20%28double-precision%29) (TriggeredSeconds :type Float%20%28double-precision%29) (InputAction :type Input%20Action%20Object%20Reference :default "/Game/Alone/Core/Input/Actions/IA_Help.IA_Help"))
  ;[1 1 1] Show/hide help panel
  (:Triggered
    (bind _foundwidgets (Widget|GetAllWidgetsOfClass "/Game/Alone/UI/HUD/W_Panel_Help.W_Panel_Help_C" true))
    (if (Utilities|Array|IsEmpty _foundwidgets)
      (bind _returnvalue (UserInterface|CreateWidget "/Game/Alone/UI/HUD/W_Panel_Help.W_Panel_Help_C"))
      (UserInterface|Viewport|AddtoViewport _returnvalue 0)
      (else
        (for _array_element _foundwidgets
          (Widget|RemovefromParent _array_element))))))

(event Input|EnhancedActionEvents|EnhancedInputActionIA_Dev_Trigger1
  (params (ActionValue :type Boolean) (ElapsedSeconds :type Float%20%28double-precision%29) (TriggeredSeconds :type Float%20%28double-precision%29) (InputAction :type Input%20Action%20Object%20Reference :default "/Game/Alone/Core/Input/DevActions/IA_Dev_Trigger1.IA_Dev_Trigger1"))
  ;[0.8796 0.552 0.004777] Dev trigger 1
  (:Triggered
    (Development|PrintString "Dev. trigger 1")
    (bind _outactors (Actor|GetAllActorswithInterface "/Game/Alone/Placeables/Spawners/BPI_Spawner.BPI_Spawner_C"))
    (for _array_element _outactors
      (Class|BPISpawner|SpawnTick(Message) _array_element))
    (Development|PrintString "Done")))

(event EventBeginPlay
  (bind _returnvalue (PlayerController|LocalPlayerSubsystems|GetEnhancedInputLocalPlayerSubsystem))
  ;[1 1 1] Define mapping contexts to use
  (Input|AddMappingContext _returnvalue "/Game/Alone/Core/Input/Mappings/IMC_Game.IMC_Game" 0 "(bIgnoreAllPressedKeysUntilRelease=True,bForceImmediately=False)")
  (Input|AddMappingContext _returnvalue "/Game/Alone/Core/Input/Mappings/IMC_Dev.IMC_Dev" 1 "(bIgnoreAllPressedKeysUntilRelease=True,bForceImmediately=False)")
  (Input|SetInputModeGameOnly self true)
  (bind _returnvalue_2 (UserInterface|CreateWidget "/Game/Alone/UI/HUD/W_HUD.W_HUD_C"))
  (UserInterface|Viewport|AddtoViewport _returnvalue_2 0))

(fn ConstructionScript)