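; BP_AloneWorldObject is a world object Blueprint whose root static mesh can be moved and spun through events.
; RelativeMove drives a Timeline forward or in reverse, adding a lerped share of the remaining relative offset each update and flagging EndMove when finished.
; Rotation starts a looping timer that turns the mesh in small steps until RotationStop clears it.
; The construction script sets physics simulation from the Save flag.
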(event Custom|Rotation%20Helper
  (Transformation|AddRelativeRotation (Variables|Default|GetRootStaticMesh) "0.000000,5.000000,0.000000" false false))

(event EventBeginPlay)

(event Collision|EventActorBeginOverlap
  (params (OtherActor :type Actor%20Object%20Reference)))

(event EventTick
  (params (DeltaSeconds :type Float%20%28single-precision%29)))

(event EventRotationStop
  (Utilities|Time|ClearandInvalidateTimerbyHandle (Variables|Default|GetTimer)))

(event EventRelativeMove
  (params (Target%20Relative%20Location :type Vector :default "0, 0, 0") (Reverse :type Boolean))
  (if Reverse
    (bind _value (Timeline|Timeline ReverseFromEnd)
      (:Update
        (Transformation|AddRelativeLocation (Variables|Default|GetRootStaticMesh) (Math|Vector|Lerp(Vector) "0, 0, 0" (Variables|Default|GetTarget%20Relative%20Location) _value) false false)
        (Variables|Default|SetTarget%20Relative%20Location (- (Variables|Default|GetTarget%20Relative%20Location) (Math|Vector|Lerp(Vector) "0, 0, 0" (Variables|Default|GetTarget%20Relative%20Location) _value))))
      (:Finished
        (Variables|Default|Setend%20Move true)))
    (else
      (Variables|Default|SetTarget%20Relative%20Location Target%20Relative%20Location)
      (Variables|Default|Setend%20Move false)
      (Timeline|Timeline PlayFromStart))))

(event EventRotation
  (bind _returnvalue (Utilities|Time|SetTimerbyEvent (delegate Custom|Rotation%20Helper) 0.05 true true))
  (Variables|Default|SetTimer _returnvalue))

(fn ConstructionScript
  (Physics|SetSimulatePhysics (Variables|Default|GetRootStaticMesh) (Variables|Default|Getsave)))