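; Animal actor for Pelea capreolus (grey rhebok) that varies its look by Adult and Female flags and plays a looping animation.
; The construction script scales adult males, adult females and juveniles differently, toggling a mesh material section for females and juveniles.
; BeginPlay repeats this except the adult male scale, but targets a different material section index, then starts the animation and prints a debug message.
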(event EventBeginPlay
  (if (Variables|Default|GetAdult)
    (if (Variables|Default|GetFemale)
      (Transformation|SetActorScale3D "0.850000,0.850000,0.850000")
      (Class|SkinnedMeshComponent|ShowMaterialSection (Variables|Default|GetSkeletalMesh) 2 0 false :!label _label))
    (else
      (Transformation|SetActorScale3D "0.500000,0.500000,0.500000")
      (goto _label)))
  (Components|Animation|PlayAnimation (Variables|Default|GetSkeletalMesh) "/Game/Alone/Models/Animals/Mammals/Palea_capreolus/SK_Pelea_capreolus_Anim.SK_Pelea_capreolus_Anim" true)
  (Development|PrintString "Animation Played"))

(event Collision|EventActorBeginOverlap
  (params (OtherActor :type Actor%20Object%20Reference)))

(event EventTick
  (params (DeltaSeconds :type Float%20%28single-precision%29)))

(fn ConstructionScript
  (if (Variables|Default|GetAdult)
    (if (Variables|Default|GetFemale)
      (Transformation|SetActorScale3D "0.850000,0.850000,0.850000")
      (Class|SkinnedMeshComponent|ShowMaterialSection (Variables|Default|GetSkeletalMesh) 3 0 false :!label _label)
      (else
        (Transformation|SetActorScale3D "1.000000,1.000000,1.000000")))
    (else
      (Transformation|SetActorScale3D "0.500000,0.500000,0.500000")
      (goto _label))))