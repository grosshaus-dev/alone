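; BP_Chest_Medium is a medium chest container that animates its lid when opened or closed.
; It overrides the Open and Close events, using MoveComponentTo on the Lid component before calling the parent implementation.
; Close moves the lid to an offset, rotated relative transform, while Open leaves the target transform at its defaults.
; All other container behavior comes from the parent class.
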(event EventBeginPlay
  (|CallParentFunction) ; This node is disabled and will not be called.\nDrag off pins to build functionality.
)

(event Collision|EventActorBeginOverlap
  (params (OtherActor :type Actor%20Object%20Reference))
  (|CallParentFunction OtherActor) ; This node is disabled and will not be called.\nDrag off pins to build functionality.
)

(event EventTick
  (params (DeltaSeconds :type Float%20%28single-precision%29))
  (|CallParentFunction DeltaSeconds) ; This node is disabled and will not be called.\nDrag off pins to build functionality.
)

(event EventOpen
  (Components|MoveComponentTo (Variables|Default|GetLid) "0, 0, 0" "0, 0, 0" false false 0.2 false)
  (|CallParentFunction))

(event EventClose
  (Components|MoveComponentTo (Variables|Default|GetLid) "0.000000,-21.000000,-13.000000" "-25.000000,0.000000,30.000000" false false 0.2 false)
  (|CallParentFunction))

(fn ConstructionScript
  (|CallParentFunction))