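; BP_Container is an interactable container that toggles between open and closed, with matching "Open"/"Close" interaction text.
; Opening waits briefly, then calls TakeOut to move three item components toward preset relative positions through an intermediate point.
; TakeOut then hands each component to Rotate, which re-calls itself to loop timed half-turns via MoveComponentTo.
; Close, also run on BeginPlay, only clears IsOpen and does not move the items back.
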(event Custom|Rotate
  (params (Component :type Scene%20Component%20Object%20Reference) (TargetRelativeLocation :type Vector))
  (Components|MoveComponentTo Component TargetRelativeLocation "0.000000,180.000000,0.000000" false false 2.0 false)
  (Components|MoveComponentTo Component TargetRelativeLocation "0.000000,0.000000,0.000000" false false 2.0 false)
  (CallFunction|Rotate Component TargetRelativeLocation))

(event Custom|Open
  (Variables|Default|SetIsOpen true)
  (Utilities|FlowControl|Delay 0.2)
  (CallFunction|TakeOut (Variables|Default|GetItemNo1) "30.000000,40.000000,30.000000")
  (CallFunction|TakeOut (Variables|Default|GetItemNo2) "40.000000,40.000000,30.000000")
  (CallFunction|TakeOut (Variables|Default|GetItemNo3) "50.000000,40.000000,30.000000"))

(event Custom|Close
  (Variables|Default|SetIsOpen false))

(event Custom|Take%20Out
  (params (Component :type Scene%20Component%20Object%20Reference) (TargetRelativeLocation :type Vector))
  (bind _output_get (Variables|Default|SetTarget%20Relative%20Location TargetRelativeLocation))
  (Components|MoveComponentTo Component (Math|Conversions|ToVector(Float) (.y _output_get)) "0, 0, 0" false false 0.2 false)
  (Components|MoveComponentTo Component TargetRelativeLocation "0, 0, 0" false false 0.2 false)
  (CallFunction|Rotate Component TargetRelativeLocation))

(event EventBeginPlay
  (CallFunction|Close))

(event EventInteract
  (if (Variables|Default|GetIsOpen)
    (CallFunction|Close)
    (else
      (CallFunction|Open))))

(fn ConstructionScript)

(fn GetAltInteractionText
  (return ""))

(fn GetInteractionText
  (if (Variables|Default|GetIsOpen)
    (return "Close")
    (else
      (return "Open"))))