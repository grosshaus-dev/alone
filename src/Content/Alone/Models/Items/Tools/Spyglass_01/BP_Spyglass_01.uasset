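; Spyglass tool item that lets the player zoom the camera through a scope overlay.
; Primary use toggles on the current camera FOV: it moves the mesh, hides the tube and glass parts, shows the overlay widget and plays the Zoom timeline, or hides the overlay and reverses it.
; The timeline drives the FOV and restores the parts at default FOV.
; Equip and end-of-use events slide the telescoping segments and reposition the root mesh.
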(event EventBeginPlay
  ;[0.15 0.15 0.15 0.5] Add overlay widget
  (bind _returnvalue (UserInterface|CreateWidget "/Game/Alone/Models/Items/Tools/Spyglass_01/W_Overlay.W_Overlay_C"))
  (bind _output_get (Variables|Default|Setoverlay _returnvalue))
  (UserInterface|Viewport|AddtoViewport _output_get 0)
  (Widget|SetVisibility _output_get "Hidden"))

(event EventPrimaryStarted
  (params (Hand :type E_Hand%20Enum :default "NewEnumerator0"))
  ;[0.15 0.15 0.15 0.5] Primary event
  (bind _asalone_player_character (Utilities|Casting|CastToAlonePlayerCharacter (Game|GetPlayerCharacter 0)))
  (if (== (Variables|/Script/Engine.CameraComponent|GetFieldOfView (Variables|/Game/Alone/Core/PlayerCharacter/AlonePlayerCharacter.AlonePlayerCharacter_C|GetCamera _asalone_player_character)) 9e+01)
    (Components|MoveComponentTo (Variables|Default|GetStaticMesh_0) "23.000000,0.000000,25.000000" "90.000000,0.000000,0.000000" true false 0.5 false)
    (Rendering|SetVisibility (Variables|Default|GetPart2) false false)
    (Variables|/Script/UMG.Widget|SetVisibility (Variables|Default|Getoverlay) "Visible")
    (bind _zoom_track (Timeline|Zoom Play)
      (:Finished
        (Camera|SetFieldOfView (Variables|/Game/Alone/Core/PlayerCharacter/AlonePlayerCharacter.AlonePlayerCharacter_C|GetCamera _asalone_player_character) (Math|Float|Lerp 9e+01 2e+01 _zoom_track))
        (if (== (Math|Float|Lerp 9e+01 2e+01 _zoom_track) 9e+01)
          (Rendering|SetVisibility (Variables|Default|GetPart2) true false)
          (Components|MoveComponentTo (Variables|Default|GetStaticMesh_0) "-10.000000,0.000000,0.000000" "30.000000,0.000000,0.000000" false false 0.2 false))))
    (else
      (Variables|/Script/UMG.Widget|SetVisibility (Variables|Default|Getoverlay) "Hidden")
      (Timeline|Zoom Reverse))))

(event EventOnEquip
  ;[0.15 0.15 0.15 0.5] Equip
  (Components|MoveComponentTo (Variables|Default|GetPart2) "0, 0, 0" "0, 0, 0" false false 0.2 false)
  (Components|MoveComponentTo (Variables|Default|GetPart3) "0, 0, 0" "0, 0, 0" false false 0.2 false)
  (Components|MoveComponentTo (Variables|Default|GetPart4) "0, 0, 0" "0, 0, 0" false false 0.2 false)
  (Components|MoveComponentTo (Variables|Default|GetRootStaticMesh) "-10.000000,0.000000,0.000000" "30.000000,0.000000,0.000000" false false 0.2 false))

(event EventEndOfUse
  ;[0.15 0.15 0.15 0.5] End Use
  (Components|MoveComponentTo (Variables|Default|GetRootStaticMesh) "0, 0, 0" "0, 0, 0" false false 0.2 false)
  (Components|MoveComponentTo (Variables|Default|GetPart4) "-0.850000,0.000000,0.000000" "0, 0, 0" false false 0.2 false)
  (Components|MoveComponentTo (Variables|Default|GetPart3) "-0.450000,0.000000,0.000000" "0, 0, 0" false false 0.2 false)
  (Components|MoveComponentTo (Variables|Default|GetPart2) "-0.450000,0.000000,0.000000" "0, 0, 0" false false 0.2 false))

(fn ConstructionScript)