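; Large ship chest container Blueprint that animates its lid and latch when opened and closed.
; PlayOpenAnimation swings the latch in two eased MoveComponentTo steps, then rotates the lid open over one second.
; PlayCloseAnimation reverses this, lowering the lid first and then returning the latch through the same intermediate angle.
; All motion is scripted component movement, with no timeline or per-tick logic in the graph.
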(event EventBeginPlay
  (|CallParentFunction) ; This node is disabled and will not be called.\nDrag off pins to build functionality.
)

(event Collision|EventActorBeginOverlap
  (params (OtherActor :type Actor%20Object%20Reference))
  (|CallParentFunction OtherActor) ; This node is disabled and will not be called.\nDrag off pins to build functionality.
)

(event EventTick
  (params (DeltaSeconds :type Float%20%28single-precision%29))
  (|CallParentFunction DeltaSeconds) ; This node is disabled and will not be called.\nDrag off pins to build functionality.
)

(event EventPlayOpenAnimation
  (bind _latch (Variables|Default|GetLatch))
  (Components|MoveComponentTo _latch "58.641522,0.000000,2.369726" "90.000000,0.000000,0.000000" false true 0.2 false)
  (Components|MoveComponentTo _latch "58.641522,0.000000,2.369726" "240.000000,0.000000,0.000000" true false 0.2 false)
  (Components|MoveComponentTo (Variables|Default|GetLid) "0, 0, 0" "120.000000,0.000000,0.000000" true true 1.0 true))

(event EventPlayCloseAnimation
  (bind _latch (Variables|Default|GetLatch))
  (Components|MoveComponentTo (Variables|Default|GetLid) "0, 0, 0" "0, 0, 0" true true 1.0 true)
  (Components|MoveComponentTo _latch "58.641522,0.000000,2.369726" "90.000000,0.000000,0.000000" false true 0.2 true)
  (Components|MoveComponentTo _latch "58.641522,0.000000,2.369726" "0, 0, 0" true false 0.2 false))

(fn ConstructionScript
  (|CallParentFunction))