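; Medium ship chest Blueprint that animates its lid and two latches opening and closing.
; PlayOpenAnimation flips the right and left latches, then swings the lid up; PlayCloseAnimation lowers the lid before resetting the latches.
; Both events chain eased, latent MoveComponentTo calls on relative rotation instead of using Timelines or animation assets.
; The file holds no other active logic beyond the parent construction script call.
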(event EventBeginPlay
  (|CallParentFunction) ; This node is disabled and will not be called.\nDrag off pins to build functionality.
)

(event Collision|EventActorBeginOverlap
  (params (OtherActor :type Actor%20Object%20Reference))
  (|CallParentFunction OtherActor) ; This node is disabled and will not be called.\nDrag off pins to build functionality.
)

(event EventTick
  (params (DeltaSeconds :type Float%20%28single-precision%29))
  (|CallParentFunction DeltaSeconds) ; This node is disabled and will not be called.\nDrag off pins to build functionality.
)

(event EventPlayOpenAnimation
  (bind _latchright (Variables|Default|GetLatchRight))
  (bind _latchleft (Variables|Default|GetLatchLeft))
  (Components|MoveComponentTo _latchright (Variables|/Script/Engine.SceneComponent|GetRelativeLocation _latchright) "-170.000000,0.000000,0.000000" true true 0.3 false)
  (Components|MoveComponentTo _latchleft (Variables|/Script/Engine.SceneComponent|GetRelativeLocation _latchleft) "-170.000000,0.000000,0.000000" true true 0.3 false)
  (Components|MoveComponentTo (Variables|Default|GetLid) "0, 0, 0" "100.000000,0.000000,0.000000" true true 1.0 true))

(event EventPlayCloseAnimation
  (bind _latchright (Variables|Default|GetLatchRight))
  (bind _latchleft (Variables|Default|GetLatchLeft))
  (Components|MoveComponentTo (Variables|Default|GetLid) "0, 0, 0" "0.000000,0.000000,0.000000" true true 1.0 true)
  (Components|MoveComponentTo _latchright (Variables|/Script/Engine.SceneComponent|GetRelativeLocation _latchright) "0.000000,0.000000,0.000000" true true 0.3 true)
  (Components|MoveComponentTo _latchleft (Variables|/Script/Engine.SceneComponent|GetRelativeLocation _latchleft) "0.000000,0.000000,0.000000" true true 0.3 true))

(fn ConstructionScript
  (|CallParentFunction))