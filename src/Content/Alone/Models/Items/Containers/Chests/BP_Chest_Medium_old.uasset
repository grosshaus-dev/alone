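; Medium chest actor, named as an old version, whose lid the player can open and close.
; Interact flips the Open flag and snaps the Lid component between a fixed closed offset and a zeroed open transform, without animation.
; BeginPlay applies the closed pose when Open is false, and the prompt text reads Open or Close to match.
; Alternate interaction is an empty stub with placeholder text, and no storage logic is present.
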(event EventBeginPlay
  (if (not (Variables|Default|GetOpen))
    (Transformation|SetRelativeLocationAndRotation (Variables|Default|GetLid) "0.000000,-21.000000,-13.000000" "0.000000,0.000000,30.000000" false false)))

(event Collision|EventActorBeginOverlap
  (params (OtherActor :type Actor%20Object%20Reference)))

(event EventTick
  (params (DeltaSeconds :type Float%20%28single-precision%29)))

(event EventInteract
  (if (Variables|Default|GetOpen)
    (Transformation|SetRelativeLocationAndRotation (Variables|Default|GetLid) "0.000000,-21.000000,-13.000000" "0.000000,0.000000,30.000000" false false)
    (Variables|Default|SetOpen false)
    (else
      (Transformation|SetRelativeLocationAndRotation (Variables|Default|GetLid) "0, 0, 0" "0, 0, 0" false false)
      (Variables|Default|SetOpen true))))

(event EventInteractAlt)

(fn ConstructionScript)

(fn GetAltInteractionText
  (return "alt"))

(fn GetInteractionText
  (if (Variables|Default|GetOpen)
    (return "Close")
    (else
      (return "Open"))))