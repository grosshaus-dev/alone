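; Base interactable container that toggles between open and closed, with interaction text matching the current state.
; Interact calls Open or Close, which update IsOpen and fire empty animation events meant for child Blueprints to implement.
; The construction script uses the Save flag to set root mesh physics simulation and actor collision.
; Moving contents in and out is described in comments but not implemented here.
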(event Custom|Open
  ;[0.15 0.15 0.15 0.5] Open the container and move the instance of object to the right place
  (if (not (Variables|Default|GetIsOpen))
    (CallFunction|PlayOpenAnimation)
    (Variables|Default|SetIsOpen true)))

(event Custom|Close
  ;[0.15 0.15 0.15 0.5] move the objects into the container and close
  (if (Variables|Default|GetIsOpen)
    (CallFunction|PlayCloseAnimation)
    (Variables|Default|SetIsOpen false)))

(event Custom|PlayOpenAnimation)

(event Custom|PlayCloseAnimation)

(event EventBeginPlay)

(event EventInteract
  ;[0.15 0.15 0.15 0.5] Interaction
  (if (Variables|Default|GetIsOpen)
    (CallFunction|Close)
    (else
      (CallFunction|Open))))

(fn ConstructionScript
  (bind _save (Variables|Default|Getsave))
  (Physics|SetSimulatePhysics (Variables|Default|GetRootStaticMesh) _save)
  (Collision|SetActorEnableCollision _save))

(fn GetAltInteractionText
  (return ""))

(fn GetInteractionText
  (if (Variables|Default|GetIsOpen)
    (return "Close")
    (else
      (return "Open"))))