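; Small ship chest container Blueprint that supplies its own open and close animations.
; Opening runs chained MoveComponentTo moves that swing the left latch, crossbar, front latch and lid in turn, and closing reverses the order back to zero rotation.
; Crossbar and lid swings pass through an intermediate angle, so shortest-path rotation can carry them beyond 180 degrees in the intended direction.
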(event EventBeginPlay
  (|CallParentFunction) ; This node is disabled and will not be called.\nDrag off pins to build functionality.
)

(event Collision|EventActorBeginOverlap
  (params (OtherActor :type Actor%20Object%20Reference))
  (|CallParentFunction OtherActor) ; This node is disabled and will not be called.\nDrag off pins to build functionality.
)

(event EventTick
  (params (DeltaSeconds :type Float%20%28single-precision%29))
  (|CallParentFunction DeltaSeconds) ; This node is disabled and will not be called.\nDrag off pins to build functionality.
)

(event EventPlayOpenAnimation
  (bind _lid (Variables|Default|GetLid))
  (bind _latchfront (Variables|Default|GetLatchFront))
  (bind _crossbar (Variables|Default|GetCrossbar))
  (bind _latchleft (Variables|Default|GetLatchLeft))
  (bind _relativelocation (Variables|/Script/Engine.SceneComponent|GetRelativeLocation _crossbar))
  (Components|MoveComponentTo _latchleft (Variables|/Script/Engine.SceneComponent|GetRelativeLocation _latchleft) "0.000000,0.000000,-140.000000" false true 0.2 true)
  (Components|MoveComponentTo _crossbar _relativelocation "0.000000,0.000000,-100.000000" false false 0.2 true)
  (Components|MoveComponentTo _crossbar _relativelocation "0.000000,0.000000,-220.000000" true false 0.2 true)
  (Components|MoveComponentTo _latchfront (Variables|/Script/Engine.SceneComponent|GetRelativeLocation _latchfront) "160.000000,0.000000,0.000000" false true 0.3 true)
  (Components|MoveComponentTo _lid "0, 0, 0" "100.000000,0.000000,0.000000" false false 0.2 true)
  (Components|MoveComponentTo _lid "0, 0, 0" "200.000000,0.000000,0.000000" true false 0.2 true))

(event EventPlayCloseAnimation
  (bind _latchleft (Variables|Default|GetLatchLeft))
  (bind _crossbar (Variables|Default|GetCrossbar))
  (bind _latchfront (Variables|Default|GetLatchFront))
  (bind _lid (Variables|Default|GetLid))
  (bind _relativelocation (Variables|/Script/Engine.SceneComponent|GetRelativeLocation _crossbar))
  (Components|MoveComponentTo _lid "0, 0, 0" "100.000000,0.000000,0.000000" false true 0.2 true)
  (Components|MoveComponentTo _lid "0, 0, 0" "0, 0, 0" false false 0.2 true)
  (Components|MoveComponentTo _latchfront (Variables|/Script/Engine.SceneComponent|GetRelativeLocation _latchfront) "0, 0, 0" true false 0.3 true)
  (Components|MoveComponentTo _crossbar _relativelocation "0.000000,0.000000,-100.000000" false true 0.2 true)
  (Components|MoveComponentTo _crossbar _relativelocation "0, 0, 0" false false 0.2 true)
  (Components|MoveComponentTo _latchleft (Variables|/Script/Engine.SceneComponent|GetRelativeLocation _latchleft) "0, 0, 0" true false 0.2 true))

(fn ConstructionScript
  (|CallParentFunction))