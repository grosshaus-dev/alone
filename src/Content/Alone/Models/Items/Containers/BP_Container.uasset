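; Base interactable container that toggles open and closed, revealing its stored items in the world, with open and close animations left to child Blueprints.
; Once the player is ready, it spawns each item, or a BP_StorageSlot for empty entries, at the Content point.
; Opening fans these actors into rows, recording offsets and adding temporary slots linked to items.
; Closing destroys those slots and reverses the offsets; removed items are replaced by empty slots.
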(event Custom|Remove%20Item
  (params (Item :type BP%20Alone%20World%20Object%20Object%20Reference))
  (bind _instanceofslots (Variables|Default|GetInstanceOfSlots))
  (bind _returnvalue (Utilities|Array|FindItem _instanceofslots Item))
  ;[0.15 0.15 0.15 0.5] take object out of container
  (Utilities|Array|RemoveIndex (Variables|Default|GetItems) _returnvalue)
  (bind _returnvalue_2 (Game|SpawnActorfromClass "/Game/Alone/Core/Inventory/BP_StorageSlot.BP_StorageSlot_C" (Math|Transform|MakeTransform (Utilities|GetAbsoluteLocation _returnvalue) "90.000000,0.000000,0.000000" "1.000000,1.000000,1.000000") "Undefined" "MultiplyWithRoot" 0 0 0 1e+02 false false 0))
  (Utilities|Array|SetArrayElem (Variables|Default|GetInstanceOfSlots) _returnvalue _returnvalue_2))

(event Custom|Open
  ;[0.15 0.15 0.15 0.5] Open the container and move the instance of object to the right place
  (CallFunction|PlayOpenAnimation)
  (Utilities|FlowControl|Delay 1.5)
  (Variables|Default|SetIsOpen true)
  (for (_array_element _array_index) (Variables|Default|GetInstanceOfSlots)
    (if (== (Math|Integer|%(Integer) _array_index (Math|Float|Truncate (Math|Float|Sqrt (Math|Conversions|ToFloat(Integer) (Variables|Default|GetsizeOfItems))))) 0)
      (if (== (Math|Integer|%(Integer) _array_index 2) 0)
        (Variables|Default|SetforOdd 0.0)
        (Variables|Default|SetforEven -3e+01)
        (Variables|Default|SetHeight (+ (Variables|Default|GetHeight) 3e+01))
        (Variables|Default|Setcounter 0)
        (else
          (Variables|Default|SetforOdd 3e+01)
          (Variables|Default|SetforEven 0.0)
          (Variables|Default|SetHeight (+ (Variables|Default|GetHeight) 3e+01))
          (Variables|Default|Setcounter 0))))
    (if (== (Math|Integer|%(Integer) _array_index 2) 0)
      (bind _output_get (Variables|Default|SetforEven (+ (Variables|Default|GetforEven) 3e+01)))
      (Class|BPIMovement|RelativeMove(Message) _array_element (Math|Vector|MakeVector 0.0 _output_get (Variables|Default|GetHeight)) false)
      (Utilities|Array|Add (Variables|Default|GetRelative%20Y) (Variables|Default|GetforEven))
      (else
        (bind _output_get_2 (Variables|Default|SetforOdd (- (Variables|Default|GetforOdd) 3e+01)))
        (Class|BPIMovement|RelativeMove(Message) _array_element (Math|Vector|MakeVector 0.0 _output_get_2 (Variables|Default|GetHeight)) false)
        (Utilities|Array|Add (Variables|Default|GetRelative%20Y) (Variables|Default|GetforOdd))))
    (bind _returnvalue (Utilities|Array|Add (Variables|Default|GetRelative%20Z) (Variables|Default|GetHeight)))
    (if (!= (Utilities|GetClass (Utilities|Array|Get(acopy) (Variables|Default|GetInstanceOfSlots) _returnvalue)) "/Game/Alone/Core/Inventory/BP_StorageSlot.BP_StorageSlot_C")
      (bind _returnvalue_2 (Game|SpawnActorfromClass "/Game/Alone/Core/Inventory/BP_StorageSlot.BP_StorageSlot_C" (Math|Transform|MakeTransform (Utilities|GetAbsoluteLocation _returnvalue) "90.000000,0.000000,0.000000" "0.100000,0.100000,0.100000") "Undefined" "MultiplyWithRoot" 0 self (Utilities|Array|Get(acopy) (Variables|Default|GetInstanceOfSlots) _returnvalue) 1e+02 false false 0))
      (Utilities|Array|Add (Variables|Default|GetToDistroy) _returnvalue_2)))
  (Variables|Default|SetforOdd 0.0)
  (Variables|Default|SetforEven -3e+01)
  (Variables|Default|SetHeight 2e+01)
  (Utilities|FlowControl|Delay 1.0)
  (Variables|Default|SetReadyToClose true))

(event Custom|Close
  ;[0.15 0.15 0.15 0.5] move the objects into the container and close
  (if (Variables|Default|GetReadyToClose)
    (Variables|Default|SetIsOpen false)
    (for _array_element (Variables|Default|GetToDistroy)
      (Utilities|IsValid _array_element
        (:Is%20Valid
          (Variables|/Game/Alone/Core/Inventory/BP_StorageSlot.BP_StorageSlot_C|SetRemovable%20Item _array_element _array_element)
          (Actor|DestroyActor _array_element))))
    (for (_array_element_2 _array_index) (Variables|Default|GetInstanceOfSlots)
      (Class|BPIMovement|RelativeMove(Message) _array_element_2 (Math|Vector|MakeVector 0.0 (* (Utilities|Array|Get(acopy) (Variables|Default|GetRelative%20Y) _array_index) -1.0) (* (Utilities|Array|Get(acopy) (Variables|Default|GetRelative%20Z) _array_index) -1.0)) false))
    (Utilities|Array|Clear (Variables|Default|GetRelative%20Y))
    (Utilities|Array|Clear (Variables|Default|GetRelative%20Z))
    (CallFunction|PlayCloseAnimation)))

(event Custom|PlayOpenAnimation)

(event Custom|PlayCloseAnimation)

(event EventBeginPlay
  (bind _content (Variables|Default|GetContent))
  (bind _returnvalue (Transformation|GetWorldLocation _content))
  ;[0.15 0.15 0.15 0.5] Spawn objects into the container
  (bind _asalone_player_character (Utilities|Casting|CastToAlonePlayerCharacter (Game|GetPlayerCharacter 0)))
  ;;[0.15 0.15 0.15 0.5] Wair for player character to be ready
  (if (Variables|/Game/Alone/Core/PlayerCharacter/AlonePlayerCharacter.AlonePlayerCharacter_C|GetReady _asalone_player_character) :!label _label
    (for _index (range 0 (- (Variables|Default|GetsizeOfItems) 1))
      (if (Utilities|IsValidClass (Utilities|Array|Get(acopy) (Variables|Default|GetItems) _index))
        (bind _returnvalue_2 (Game|SpawnActorfromClass (Utilities|Array|Get(acopy) (Variables|Default|GetItems) _index) (Math|Transform|MakeTransform _returnvalue "90.000000,0.000000,0.000000" "1.000000,1.000000,1.000000") "AlwaysSpawn" "MultiplyWithRoot" 0 1e+02 false false 0))
        (Utilities|Array|Add (Variables|Default|GetInstanceOfSlots) _returnvalue_2)
        (else
          (bind _returnvalue_3 (Game|SpawnActorfromClass "/Game/Alone/Core/Inventory/BP_StorageSlot.BP_StorageSlot_C" (Math|Transform|MakeTransform _returnvalue "90.000000,0.000000,0.000000" "1.000000,1.000000,1.000000") "AlwaysSpawn" "MultiplyWithRoot" 0 0 0 1e+02 false false 0))
          (Utilities|Array|Add (Variables|Default|GetInstanceOfSlots) _returnvalue_3))))
    (else
      (Utilities|FlowControl|Delay 0.2)
      (goto _label))))

(event EventInteract
  ;[0.15 0.15 0.15 0.5] Interaction
  (if (Variables|Default|GetIsOpen)
    (CallFunction|Close)
    (else
      (CallFunction|Open))))

(fn ConstructionScript)

(fn GetAltInteractionText
  (return ""))

(fn GetInteractionText
  (if (Variables|Default|GetIsOpen)
    (return "Close")
    (else
      (return "Open"))))