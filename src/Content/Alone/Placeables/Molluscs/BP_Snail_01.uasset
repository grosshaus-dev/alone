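; BP_Snail_01 is a placeable snail that crawls forward with looping foot and shell animations while alive and open.
; Tick steadily interpolates its rotation toward a target derived from its forward and right vectors, and moves it without sweeping.
; Equipping flips the shell and closes it, swapping foot for cap and stopping animation; unequipping reverses this.
; Open, Close and Die extend parent behavior, with death hiding foot and cap.
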(event EventBeginPlay
  (CallFunction|StartAnimation))

(event EventTick
  (params (DeltaSeconds :type Float%20%28single-precision%29))
  (CallFunction|Rotate DeltaSeconds)
  (CallFunction|Move DeltaSeconds))

(event EventOnUnequip
  (Transformation|SetRelativeRotation (Variables|Default|GetShell) "0.000000,0.000000,0.000000" false false)
  (CallFunction|Open))

(event EventOnEquip
  (Transformation|SetRelativeRotation (Variables|Default|GetShell) "180.000000,0.000000,0.000000" false false)
  (CallFunction|Close))

(fn ConstructionScript
  (Utilities|FlowControl|Sequence
    (:then_1
      (if (Variables|Default|Getalive)
        (if (Variables|Default|Getclosed)
          (Rendering|SetVisibility (Variables|Default|GetFoot) false false)
          (else
            (Rendering|SetVisibility (Variables|Default|GetCap) false false :!label _label)))
        (else
          (goto _label))))))

(fn Close
  (|CallParentFunction)
  (if (Variables|Default|Getalive)
    (Variables|Default|Setclosed true)
    (CallFunction|StopAnimation)
    (Rendering|SetVisibility (Variables|Default|GetFoot) false false)
    (Rendering|SetVisibility (Variables|Default|GetCap) true false)
    (else
      (return))))

(fn StopAnimation
  (Audio|Components|Audio|Stop (Variables|Default|GetFoot))
  (Audio|Components|Audio|Stop (Variables|Default|GetShell)))

(fn StartAnimation
  (Components|Animation|PlayAnimation (Variables|Default|GetFoot) "/Game/Alone/Models/Animals/Snails/Snail_01/AS_Snail_01_Foot_Anim_CrawlSimpleAction.AS_Snail_01_Foot_Anim_CrawlSimpleAction" true)
  (Components|Animation|PlayAnimation (Variables|Default|GetShell) "/Game/Alone/Models/Animals/Snails/Snail_01/AS_Snail_01_Shell_Anim_CrawlSimpleAction.AS_Snail_01_Shell_Anim_CrawlSimpleAction" true))

(fn Die
  (|CallParentFunction)
  (Variables|Default|Setalive false)
  (CallFunction|StopAnimation)
  (Rendering|SetVisibility (Variables|Default|GetCap) false false))

(fn Open
  (|CallParentFunction)
  (if (Variables|Default|Getalive)
    (Variables|Default|Setclosed false)
    (CallFunction|StartAnimation)
    (Rendering|SetVisibility (Variables|Default|GetCap) false false)
    (Rendering|SetVisibility (Variables|Default|GetFoot) true false)
    (else
      (return))))

(fn Rotate
  (params (DeltaSeconds :type Float%20%28double-precision%29))
  (bind _self self)
  (Transformation|SetActorRotation (Class|KismetMathLibrary|RInterptoConstant (Transformation|GetActorRotation self) (Math|Rotator|FindLookatRotation (Transformation|GetActorForwardVector _self) (Transformation|GetActorRightVector _self)) DeltaSeconds 1.0)))

(fn Move
  (params (DeltaSeconds :type Float%20%28double-precision%29))
  (bind _self self)
  ;[1 1 1] Move forward
  (if (Variables|Default|Getalive)
    (if (not (Variables|Default|Getclosed))
      (Transformation|SetActorLocation (+ (Transformation|GetActorLocation _self) (* (Transformation|GetActorForwardVector _self) DeltaSeconds)) false false))))