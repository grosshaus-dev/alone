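; Alikreukel sea snail placeable that crawls slowly forward while alive and open.
; Tick turns it at a constant rate toward a look-at rotation derived from its forward and right vectors, even when closed or dead.
; Open, Close and Die extend parent behavior by toggling Foot and Cap visibility and starting or stopping looping Foot and Shell crawl animations.
; The construction script sets initial part visibility from Alive and Closed.
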(event EventBeginPlay
  (CallFunction|StartAnimation))

(event EventTick
  (params (DeltaSeconds :type Float%20%28single-precision%29))
  (CallFunction|Rotate DeltaSeconds)
  (CallFunction|Move DeltaSeconds))

(fn ConstructionScript
  (if (Variables|Default|Getalive)
    (if (Variables|Default|Getclosed)
      (Rendering|SetVisibility (Variables|Default|GetFoot) false false)
      (else
        (Rendering|SetVisibility (Variables|Default|GetCap) false false :!label _label)))
    (else
      (goto _label))))

(fn Close
  (|CallParentFunction)
  (Variables|Default|Setclosed true)
  (CallFunction|StopAnimation)
  (Rendering|SetVisibility (Variables|Default|GetFoot) false false)
  (Rendering|SetVisibility (Variables|Default|GetCap) true false))

(fn StopAnimation
  (Audio|Components|Audio|Stop (Variables|Default|GetFoot))
  (Audio|Components|Audio|Stop (Variables|Default|GetShell)))

(fn StartAnimation
  (Components|Animation|PlayAnimation (Variables|Default|GetFoot) "/Game/Alone/Models/Animals/Snails/Snail_1/snail_1_Foot_Anim_CrawlSimpleAction.snail_1_Foot_Anim_CrawlSimpleAction" true)
  (Components|Animation|PlayAnimation (Variables|Default|GetShell) "/Game/Alone/Models/Animals/Snails/Snail_1/snail_1_Shell_Anim_CrawlSimpleAction.snail_1_Shell_Anim_CrawlSimpleAction" true))

(fn Die
  (|CallParentFunction)
  (Variables|Default|Setalive false)
  (CallFunction|StopAnimation)
  (Rendering|SetVisibility (Variables|Default|GetCap) false false))

(fn Open
  (|CallParentFunction)
  (Variables|Default|Setclosed false)
  (CallFunction|StartAnimation)
  (Rendering|SetVisibility (Variables|Default|GetCap) false false)
  (Rendering|SetVisibility (Variables|Default|GetFoot) true false))

(fn Rotate
  (params (DeltaSeconds :type Float%20%28double-precision%29))
  (bind _self self)
  (Transformation|SetActorRotation (Class|KismetMathLibrary|RInterptoConstant (Transformation|GetActorRotation self) (Math|Rotator|FindLookatRotation (Transformation|GetActorForwardVector _self) (Transformation|GetActorRightVector _self)) DeltaSeconds 1.0)))

(fn Move
  (params (DeltaSeconds :type Float%20%28double-precision%29))
  (bind _self self)
  ;[1 1 1] Move forward
  (if (Variables|Default|Getalive)
    (if (not (Variables|Default|Getclosed))
      (Transformation|SetActorLocation (+ (Transformation|GetActorLocation _self) (* (Transformation|GetActorForwardVector _self) DeltaSeconds)) false false))))