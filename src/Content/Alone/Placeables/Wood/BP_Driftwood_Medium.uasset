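; BP_Driftwood_Medium is a placeable medium driftwood piece that the player can take or set alight.
; Interact destroys the actor and sends the player character a message naming this driftwood with an amount of one.
; InteractAlt prints the display name and calls Ignite, while its prompt reads "Ignite", or "(Charred)" once IsCharred is set.
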(event EventBeginPlay)

(event Collision|EventActorBeginOverlap
  (params (OtherActor :type Actor%20Object%20Reference)))

(event EventTick
  (params (DeltaSeconds :type Float%20%28single-precision%29)))

(event EventInteract
  (Actor|DestroyActor)
  (Class|BPIPlayerCharacter|Receive(Message) (Game|GetPlayerCharacter 0) "BP_Driftwood_Medium_C" 1))

(event EventInteractAlt
  (Development|PrintString (Utilities|GetDisplayName self))
  (CallFunction|Ignite 3))

(fn ConstructionScript)

(fn GetAltInteractionText
  (if (Variables|Default|GetIsCharred)
    (return "(Charred)")
    (else
      (return "Ignite"))))

(fn GetInteractionText
  (return "take"))