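; BP_Driftwood_Large is a large driftwood placeable that the player can ignite through interaction.
; Interact prints the object's display name and calls Ignite with a fixed value; Ignite's logic and the IsCharred state are not defined in this graph.
; The interaction prompt reads "Ignite", or "(Charred)" once IsCharred is set, and the alternate prompt is empty.
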(event Collision|EventActorBeginOverlap
  (params (OtherActor :type Actor%20Object%20Reference)))

(event EventTick
  (params (DeltaSeconds :type Float%20%28single-precision%29)))

(event EventInteract
  (Development|PrintString (Utilities|GetDisplayName self))
  (CallFunction|Ignite 3))

(fn ConstructionScript)

(fn GetAltInteractionText
  (return ""))

(fn GetInteractionText
  (if (Variables|Default|GetIsCharred)
    (return "(Charred)")
    (else
      (return "Ignite"))))