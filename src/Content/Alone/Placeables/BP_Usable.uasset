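; BP_Usable is a placeable item that the player can take into inventory or equip for use.
; Take and Use interactions message the player character, with Take also destroying the actor.
; With HasProgress set, holding the primary action on a BPI_Flammable actor shows progress while a timeline zooms the camera and moves the equipment.
; Repeated camera line traces cancel the action if the target changes; completion only resets progress and zoom, igniting nothing here.
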(event Custom|Parent:%20PrimaryStarted
  (if (Variables|Default|GethasProgress)
    (bind (_actorref _hastrace) (CallFunction|ActionTrace))
    (Variables|Default|SetTheHitActor _actorref)
    (if _hastrace
      (Variables|Default|SetIsNotStoped true)
      (Class|BPIPlayerCharacter|Progress(Message) (Game|GetPlayerCharacter 0) 0.0 true)
      (bind (_direction _zoom_track _location_track) (Timeline|Zoom%20Timeline Play)
        (:Update
          (bind _asalone_player_character (Utilities|Casting|CastToAlonePlayerCharacter (Game|GetPlayerCharacter 0)))
          (Camera|SetFieldOfView (Variables|/Game/Alone/Core/PlayerCharacter/AlonePlayerCharacter.AlonePlayerCharacter_C|GetCamera _asalone_player_character) (Math|Float|Lerp 9e+01 4e+01 _zoom_track))
          (Transformation|SetRelativeLocation (Variables|/Game/Alone/Core/PlayerCharacter/AlonePlayerCharacter.AlonePlayerCharacter_C|GetEquipment _asalone_player_character) _location_track false false))))))

(event Custom|Parent:%20Primary%20Triggered
  (bind (_actorref _hastrace) (CallFunction|ActionTrace))
  (if (not (and (== _actorref (Variables|Default|GetTheHitActor)) _hastrace))
    (CallFunction|PrimaryCanceled)))

(event EventBeginPlay)

(event EventInteract
  (Actor|DestroyActor)
  (Class|BPIPlayerCharacter|Receive(Message) (Game|GetPlayerCharacter 0) (Utilities|GetClass self) false 1 (Variables|Default|GetInventory%20Icon)))

(event EventTick
  (params (DeltaSeconds :type Float%20%28single-precision%29)))

(event EventInteractAlt
  (Class|BPIPlayerCharacter|Equip(Message) (Game|GetPlayerCharacter 0) self))

(event EventPrimaryCanceled
  (Variables|Default|SetIsNotStoped false)
  (if (Variables|Default|GethasProgress)
    (Class|BPIPlayerCharacter|Progress(Message) (Game|GetPlayerCharacter 0) 0.0 false)
    (bind (_direction _zoom_track _location_track) (Timeline|Zoom%20Timeline Reverse)
      (:Update
        (bind _asalone_player_character (Utilities|Casting|CastToAlonePlayerCharacter (Game|GetPlayerCharacter 0)))
        (Camera|SetFieldOfView (Variables|/Game/Alone/Core/PlayerCharacter/AlonePlayerCharacter.AlonePlayerCharacter_C|GetCamera _asalone_player_character) (Math|Float|Lerp 9e+01 4e+01 _zoom_track))
        (Transformation|SetRelativeLocation (Variables|/Game/Alone/Core/PlayerCharacter/AlonePlayerCharacter.AlonePlayerCharacter_C|GetEquipment _asalone_player_character) _location_track false false)))))

(event Collision|EventActorBeginOverlap
  (params (OtherActor :type Actor%20Object%20Reference)))

(event EventPrimaryOngoing
  (params (Elapsed%20Seconds :type Float%20%28double-precision%29))
  (if (and (Variables|Default|GethasProgress) (Variables|Default|GetIsNotStoped))
    (bind (_actorref _hastrace) (CallFunction|ActionTrace))
    (if (and (== _actorref (Variables|Default|GetTheHitActor)) _hastrace)
      (Class|BPIPlayerCharacter|Progress(Message) (Game|GetPlayerCharacter 0) Elapsed%20Seconds true)
      (else
        (CallFunction|PrimaryCanceled)))))

(event EventPrimaryCompleted
  (if (and (Variables|Default|GethasProgress) (Variables|Default|GetIsNotStoped))
    (Utilities|FlowControl|Delay 0.5)
    (Class|BPIPlayerCharacter|Progress(Message) (Game|GetPlayerCharacter 0) 0.0 false)
    (Variables|Default|SetIsNotStoped false)
    (bind (_direction _zoom_track _location_track) (Timeline|Zoom%20Timeline Reverse)
      (:Update
        (bind _asalone_player_character (Utilities|Casting|CastToAlonePlayerCharacter (Game|GetPlayerCharacter 0)))
        (Camera|SetFieldOfView (Variables|/Game/Alone/Core/PlayerCharacter/AlonePlayerCharacter.AlonePlayerCharacter_C|GetCamera _asalone_player_character) (Math|Float|Lerp 9e+01 4e+01 _zoom_track))
        (Transformation|SetRelativeLocation (Variables|/Game/Alone/Core/PlayerCharacter/AlonePlayerCharacter.AlonePlayerCharacter_C|GetEquipment _asalone_player_character) _location_track false false)))))

(fn ConstructionScript)

(fn ActionTrace
  (bind _returnvalue (Game|GetPlayerCameraManager 0))
  (bind _rootcomponent (Variables|/Script/Engine.Actor|GetRootComponent _returnvalue))
  (bind _returnvalue_2 (Transformation|GetWorldLocation _rootcomponent))
  (bind (_outhit _returnvalue_3) (Collision|LineTraceForObjects _returnvalue_2 (+ _returnvalue_2 (* (Math|Vector|GetForwardVector (Transformation|GetWorldRotation _rootcomponent)) (LocalVariables|GetReach))) (LocalVariables|GetObject%20Types) false 0 "None"))
  (Development|PrintString "call ActionTrace")
  (return (.hitactor _outhit) (and (Utilities|DoesObjectImplementInterface (.hitactor _outhit) "/Game/Alone/Core/Fire/BPI_Flammable.BPI_Flammable_C") _returnvalue_3)))

(fn GetAltInteractionText
  (return "Use"))

(fn GetInteractionText
  (return "Take"))