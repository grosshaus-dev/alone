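; BP_Magnifier is a fire-starting utensil, the magnifying glass, that ignites the actor it targets.
; On primary trigger, if IsFinished is set, it sends IgniteMessage with a fixed value to TheHitActor.
; Primary start only forwards to the parent, calling it twice in a row, and the construction script just runs the parent's.
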(event EventBeginPlay
  (|CallParentFunction) ; This node is disabled and will not be called.\nDrag off pins to build functionality.
)

(event Collision|EventActorBeginOverlap
  (params (OtherActor :type Actor%20Object%20Reference))
  (|CallParentFunction OtherActor) ; This node is disabled and will not be called.\nDrag off pins to build functionality.
)

(event EventTick
  (params (DeltaSeconds :type Float%20%28single-precision%29))
  (|CallParentFunction DeltaSeconds) ; This node is disabled and will not be called.\nDrag off pins to build functionality.
)

(event EventPrimaryTriggered
  (params (Elapsed%20Seconds :type Float%20%28double-precision%29) (Triggered%20Seconds :type Float%20%28double-precision%29))
  (if (Variables|Default|GetIsFinished)
    (Class|BPIFlammable|Ignite(Message) (Variables|Default|GetTheHitActor) 3)))

(event EventPrimaryStarted
  (CallFunction|Parent:PrimaryStarted)
  (CallFunction|Parent:PrimaryStarted))

(fn ConstructionScript
  (|CallParentFunction))