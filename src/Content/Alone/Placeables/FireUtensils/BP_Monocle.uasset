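; BP_Monocle is a fire utensil that ignites the actor it targets, usable only while the player is out of shade.
; It overrides the primary-action Started and Triggered events, calling the parent logic only if the player character's IsInShade flag is false.
; While triggered and IsNotStoped is set, it sends IgniteMessage to TheHitActor, leaving the ignition response to that actor.
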(event EventBeginPlay
  (|CallParentFunction) ; This node is disabled and will not be called.\nDrag off pins to build functionality.
)

(event Collision|EventActorBeginOverlap
  (params (OtherActor :type Actor%20Object%20Reference))
  (|CallParentFunction OtherActor) ; This node is disabled and will not be called.\nDrag off pins to build functionality.
)

(event EventTick
  (params (DeltaSeconds :type Float%20%28single-precision%29))
  (|CallParentFunction DeltaSeconds) ; This node is disabled and will not be called.\nDrag off pins to build functionality.
)

(event EventPrimaryTriggered
  (params (Elapsed%20Seconds :type Float%20%28double-precision%29) (Triggered%20Seconds :type Float%20%28double-precision%29))
  (bind _asalone_player_character (Utilities|Casting|CastToAlonePlayerCharacter (Game|GetPlayerCharacter 0)))
  (if (!= (Variables|/Game/Alone/Core/PlayerCharacter/AlonePlayerCharacter.AlonePlayerCharacter_C|GetIsInShade _asalone_player_character) true)
    (CallFunction|Parent:PrimaryTriggered)
    (if (Variables|Default|GetIsNotStoped)
      (Class|BPIFlammable|Ignite(Message) (Variables|Default|GetTheHitActor) 2))))

(event EventPrimaryStarted
  (bind _asalone_player_character (Utilities|Casting|CastToAlonePlayerCharacter (Game|GetPlayerCharacter 0)))
  (if (!= (Variables|/Game/Alone/Core/PlayerCharacter/AlonePlayerCharacter.AlonePlayerCharacter_C|GetIsInShade _asalone_player_character) true)
    (CallFunction|Parent:PrimaryStarted)))

(fn ConstructionScript
  (|CallParentFunction))