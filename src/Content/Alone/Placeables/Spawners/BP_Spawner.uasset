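; Spawner placeable that, on each SpawnTick call, may spawn randomly chosen actor classes once its spawn interval has elapsed.
; It builds a weighted pool by repeating each class per its likeliness count.
; If its sphere overlaps no actors and a chance roll passes, every spawn slot gets a random pick with random yaw, ignoring collision.
; LastSpawnTimePoint is read but never updated in this graph.
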(event EventSpawnTick
  (params (TimePoint :type Integer))
  ;[1 1 1] Check if spawn allowed
  (if (>= (- TimePoint (Variables|Default|GetLastSpawnTimePoint)) (Variables|Default|GetSpawnInterval))
    (Utilities|Array|Clear (Variables|Default|GetSpawnActorsPool))
    ;[1 1 1] Create pool of actors to spawn from
    (for (_array_element _array_index) (Variables|Default|GetSpawnLikeliness)
      (for _index (range 1 _array_element)
        (Utilities|Array|Add (Variables|Default|GetSpawnActorsPool) (Utilities|Array|Get(acopy) (Variables|Default|GetSpawnActors) _array_index))))
    ;[1 1 1] Check if spawn blocked
    (if (Utilities|Array|IsEmpty (Collision|GetOverlappingActors (Variables|Default|GetSphere) 0 :!class /Script/Engine.PrimitiveComponent))
      ;[1 1 1] Spawn chance
      (if (Math|Random|RandomBoolwithWeight (Variables|Default|GetSpawnChance))
        ;[1 1 1] Spawn actors
        (for _array_element_2 (Variables|Default|GetSpawnSlots)
          (Game|SpawnActorfromClass (.OutItem (Utilities|Array|Random (Variables|Default|GetSpawnActorsPool))) (Math|Transform|MakeTransform _array_element_2 (Math|Rotator|MakeRotator 0.0 0.0 (.yaw (Math|Random|RandomRotator false))) "1.000000,1.000000,1.000000") "AlwaysSpawn" 0 0))))))

(fn ConstructionScript)