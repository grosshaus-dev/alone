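; BP_OystercatcherNest is a placeable oystercatcher nest that varies its contents at random.
; The Construction Script flips a separate random bool for each of three child actor components and destroys those that roll true, leaving zero to three.
; The roll is unseeded, so the result can change whenever construction reruns.
; The event graph has no active logic.
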(event EventBeginPlay)

(event Collision|EventActorBeginOverlap
  (params (OtherActor :type Actor%20Object%20Reference)))

(event EventTick
  (params (DeltaSeconds :type Float%20%28single-precision%29)))

(fn ConstructionScript
  (Utilities|FlowControl|Sequence
    (:then_0
      (if (Math|Random|RandomBool)
        (Components|DestroyComponent (Variables|Default|GetChildActor))))
    (:then_1
      (if (Math|Random|RandomBool)
        (Components|DestroyComponent (Variables|Default|GetChildActor1))))
    (:then_2
      (if (Math|Random|RandomBool)
        (Components|DestroyComponent (Variables|Default|GetChildActor2))))))