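; BP_Consumable is a placeable item that the player eats or drinks through the alternate interaction (Q).
; InteractAlt destroys the actor and passes its EatValue and DrinkValue to player character 0 through EatMessage and DrinkMessage.
; Two getters supply the primary and alternate interaction text, though only the alternate interaction has logic in this graph.
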(event EventInteractAlt
  (bind _returnvalue (Game|GetPlayerCharacter 0))
  (Actor|DestroyActor)
  (Class|BPIPlayerCharacter|Eat(Message) _returnvalue (Variables|Default|GetEatValue))
  (Class|BPIPlayerCharacter|Drink(Message) _returnvalue (Variables|Default|GetDrinkValue)))

(fn ConstructionScript)

(fn GetAltInteractionText
  (return (Variables|Default|GetAlternative%20Interaction%20Text)))

(fn GetInteractionText
  (return (Variables|Default|GetInteraction%20Text)))